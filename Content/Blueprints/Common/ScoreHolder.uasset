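; ScoreHolder is an actor that puts a player's score bar on screen through a W_PlayerScore widget created at BeginPlay.
; Its world Y sign selects player 1 or player 2, with positive Y moving the bar to the right side.
; Under Balanca_GameMode the bar shows summed RoundData scores against the match maximum; other modes use round score over round points.
; Non-multiplayer games seed it from GameInstance_BAL totals, and ClearScore empties it.
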(event Custom|SetPlayerScore
  ;[0.1546 1 0] Single plauer counting based on total points match
  (Utilities|Casting|CastToBalanca_GameMode (Game|GetGameMode)
    (:then
      (bind _asgame_instance_bal (Utilities|Casting|CastToGameInstance_BAL (Game|GetGameInstance)))
      (Variables|Default|SetTotalP1Score 0)
      (Variables|Default|SetTotalP2Score 0)
      (for _array_element (Variables|/Game/Blueprints/Common/GameInstance_BAL.GameInstance_BAL_C|GetRoundData _asgame_instance_bal)
        (Variables|Default|SetTotalP1Score (+ (Variables|Default|GetTotalP1Score) (.player1Score (Utilities|Struct|BreakRoundData _array_element))))
        (Variables|Default|SetTotalP2Score (+ (Variables|Default|GetTotalP2Score) (.player2Score (Utilities|Struct|BreakRoundData _array_element))))
        (Default|SetPercent (Variables|Default|GetplayerScore) (Math|Float|SelectFloat (/ (Math|Conversions|ToFloat(Integer) (Variables|Default|GetTotalP1Score)) (Math|Conversions|ToFloat(Integer) (* (.number_of_rounds (Utilities|Struct|BreakMatchData (Variables|/Game/Blueprints/Common/GameInstance_BAL.GameInstance_BAL_C|GetMatchData _asgame_instance_bal))) (+ (.coop_points (Utilities|Struct|BreakMatchData (Variables|/Game/Blueprints/Common/GameInstance_BAL.GameInstance_BAL_C|GetMatchData _asgame_instance_bal))) (.no_coop_points (Utilities|Struct|BreakMatchData (Variables|/Game/Blueprints/Common/GameInstance_BAL.GameInstance_BAL_C|GetMatchData _asgame_instance_bal))))))) (/ (Math|Conversions|ToFloat(Integer) (Variables|Default|GetTotalP2Score)) (Math|Conversions|ToFloat(Integer) (* (.number_of_rounds (Utilities|Struct|BreakMatchData (Variables|/Game/Blueprints/Common/GameInstance_BAL.GameInstance_BAL_C|GetMatchData _asgame_instance_bal))) (+ (.coop_points (Utilities|Struct|BreakMatchData (Variables|/Game/Blueprints/Common/GameInstance_BAL.GameInstance_BAL_C|GetMatchData _asgame_instance_bal))) (.no_coop_points (Utilities|Struct|BreakMatchData (Variables|/Game/Blueprints/Common/GameInstance_BAL.GameInstance_BAL_C|GetMatchData _asgame_instance_bal))))))) (< (.Y (Math|Vector|BreakVector (Transformation|GetWorldLocation (Variables|Default|GetDefaultSceneRoot)))) 0.0)))))
    (:CastFailed
      ;[1 0.04969 0] Mp counting based on total round points
      (bind _asgame_instance_bal_2 (Utilities|Casting|CastToGameInstance_BAL (Game|GetGameInstance)))
      (Default|SetPercent (Variables|Default|GetplayerScore) (Math|Float|SelectFloat (/ (Math|Conversions|ToFloat(Integer) (Variables|/Game/Blueprints/Common/GameInstance_BAL.GameInstance_BAL_C|GetP1RoundScore _asgame_instance_bal_2)) (Math|Conversions|ToFloat(Integer) (Variables|/Game/Blueprints/Common/GameInstance_BAL.GameInstance_BAL_C|GetRoundPoints _asgame_instance_bal_2))) (/ (Math|Conversions|ToFloat(Integer) (Variables|/Game/Blueprints/Common/GameInstance_BAL.GameInstance_BAL_C|GetP2RoundScore _asgame_instance_bal_2)) (Math|Conversions|ToFloat(Integer) (Variables|/Game/Blueprints/Common/GameInstance_BAL.GameInstance_BAL_C|GetRoundPoints _asgame_instance_bal_2))) (< (.Y (Math|Vector|BreakVector (Transformation|GetWorldLocation (Variables|Default|GetDefaultSceneRoot)))) 0.0))))))

(event Custom|Clear%20Score
  (Default|SetPercent (Variables|Default|GetplayerScore) 0.0))

(event EventBeginPlay
  (bind _asgame_instance_bal (Utilities|Casting|CastToGameInstance_BAL (Game|GetGameInstance)))
  (if (Variables|/Game/Blueprints/Common/GameInstance_BAL.GameInstance_BAL_C|GetMultiplayer _asgame_instance_bal)
    _
    (else
      (Variables|Default|SetP1InitialScore (/ (Math|Conversions|ToFloat(Integer) (Variables|/Game/Blueprints/Common/GameInstance_BAL.GameInstance_BAL_C|GetP1TotalScore _asgame_instance_bal)) (Math|Conversions|ToFloat(Integer) (* (.number_of_rounds (Utilities|Struct|BreakMatchData (Variables|/Game/Blueprints/Common/GameInstance_BAL.GameInstance_BAL_C|GetMatchData _asgame_instance_bal))) (+ (.coop_points (Utilities|Struct|BreakMatchData (Variables|/Game/Blueprints/Common/GameInstance_BAL.GameInstance_BAL_C|GetMatchData _asgame_instance_bal))) (.no_coop_points (Utilities|Struct|BreakMatchData (Variables|/Game/Blueprints/Common/GameInstance_BAL.GameInstance_BAL_C|GetMatchData _asgame_instance_bal))))))))
      (Variables|Default|SetP2InitialScore (/ (Math|Conversions|ToFloat(Integer) (Variables|/Game/Blueprints/Common/GameInstance_BAL.GameInstance_BAL_C|GetP2TotalScore _asgame_instance_bal)) (Math|Conversions|ToFloat(Integer) (* (.number_of_rounds (Utilities|Struct|BreakMatchData (Variables|/Game/Blueprints/Common/GameInstance_BAL.GameInstance_BAL_C|GetMatchData _asgame_instance_bal))) (+ (.coop_points (Utilities|Struct|BreakMatchData (Variables|/Game/Blueprints/Common/GameInstance_BAL.GameInstance_BAL_C|GetMatchData _asgame_instance_bal))) (.no_coop_points (Utilities|Struct|BreakMatchData (Variables|/Game/Blueprints/Common/GameInstance_BAL.GameInstance_BAL_C|GetMatchData _asgame_instance_bal))))))))))
  (bind _returnvalue (UserInterface|CreateWidget "/Game/HUD/W_PlayerScore.W_PlayerScore_C"))
  (Variables|Default|SetplayerScore _returnvalue)
  (if (> (.Y (Math|Vector|BreakVector (Transformation|GetWorldLocation (Variables|Default|GetDefaultSceneRoot)))) 0.0)
    (Utilities|AdjustScoretoRight)
    (Progress|SetPercent (Variables|/Game/HUD/W_PlayerScore.W_PlayerScore_C|GetPB_Score (Variables|Default|GetplayerScore)) (Variables|Default|GetP2InitialScore))
    (else
      (Progress|SetPercent (Variables|/Game/HUD/W_PlayerScore.W_PlayerScore_C|GetPB_Score (Variables|Default|GetplayerScore)) (Variables|Default|GetP1InitialScore))))
  ;[0.1546 1 0] Single plauer counting based on total points match
  (UserInterface|Viewport|AddtoViewport (Variables|Default|GetplayerScore) 0))

(event Collision|EventActorBeginOverlap
  (params (OtherActor :type Actor%20Object%20Reference))
  ;[0.1546 1 0] Single plauer counting based on total points match
)

(event EventTick
  (params (DeltaSeconds :type Float%20%28single-precision%29))
  ;[0.1546 1 0] Single plauer counting based on total points match
)

(fn ConstructionScript)