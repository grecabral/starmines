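; Curtain actor that moves away and destroys itself once preparation ends.
; On BeginPlay it binds to Balanca_GameMode's preparation-over dispatcher, or, if that cast fails, to GameInstance_BAL's other-player-recipient-done dispatcher.
; Either event starts a five-second lifespan and opens a gate, through which Tick eases the actor's Y position toward a fixed target with VInterpTo.
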(event Custom|Curtain%20Drop
  (params (OtherPlayerFinalPosition :type Integer))
  (bind _returnvalue (Transformation|GetActorLocation))
  (bind (_x _y _z) (Math|Vector|BreakVector _returnvalue))
  ;[1 1 1] Curtain Fall
  (Actor|SetLifeSpan 5.0)
  (Utilities|FlowControl|Gate true) ; enters at Open
)

(event Custom|Close%20Gate
  (bind _returnvalue (Transformation|GetActorLocation))
  (bind (_x _y _z) (Math|Vector|BreakVector _returnvalue))
  (Utilities|FlowControl|Gate true) ; enters at Close
)

(event Custom|Curtain%20Drop%20SP
  (bind _returnvalue (Transformation|GetActorLocation))
  (bind (_x _y _z) (Math|Vector|BreakVector _returnvalue))
  (Actor|SetLifeSpan 5.0)
  (Utilities|FlowControl|Gate true) ; enters at Open
)

(event EventBeginPlay
  (bind _asbalanca_game_mode (Utilities|Casting|CastToBalanca_GameMode (Game|GetGameMode))
    (:then
      (EventDispatchers|BindEventtoPreparationOverDispatcher _asbalanca_game_mode (delegate Custom|Curtain%20Drop%20SP)))
    (:CastFailed
      (bind _asgame_instance_bal (Utilities|Casting|CastToGameInstance_BAL (Game|GetGameInstance)))
      (EventDispatchers|BindEventtoOtherplayerRecipientDone _asgame_instance_bal (delegate Custom|Curtain%20Drop)))))

(event EventTick
  (params (DeltaSeconds :type Float%20%28single-precision%29))
  (bind _returnvalue (Transformation|GetActorLocation))
  (bind (_x _y _z) (Math|Vector|BreakVector _returnvalue))
  (Utilities|FlowControl|Gate true
    (:Exit
      (Transformation|SetActorLocation (Math|Interpolation|VInterpTo _returnvalue (Math|Vector|MakeVector _x 1.5e+03 _z) DeltaSeconds 3.0) false false))))

(fn ConstructionScript)