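; HandActor is an actor that swings its Hand component back and forth in a continuous oscillation.
; BeginPlay records the start time and opens a gate that Tick enters every frame.
; Each pass sets the Hand's relative pitch from a sine of the elapsed time, leaving roll and yaw unchanged.
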(event Collision|EventActorBeginOverlap
  (params (OtherActor :type Actor%20Object%20Reference)))

(event EventBeginPlay
  (bind _hand (Variables|Default|GetHand))
  (bind _relativerotation (Variables|/Script/Engine.SceneComponent|GetRelativeRotation _hand))
  (bind (_roll _pitch _yaw) (Math|Rotator|BreakRotator _relativerotation))
  ;[1 1 1] Moves The Hand to right and left
  (Variables|Default|SetStartTime (Utilities|Time|GetTimeSeconds))
  (Utilities|FlowControl|Gate true) ; enters at Open
)

(event EventTick
  (params (DeltaSeconds :type Float%20%28single-precision%29))
  (bind _hand (Variables|Default|GetHand))
  (bind _relativerotation (Variables|/Script/Engine.SceneComponent|GetRelativeRotation _hand))
  (bind (_roll _pitch _yaw) (Math|Rotator|BreakRotator _relativerotation))
  ;[1 1 1] Moves The Hand to right and left
  (Utilities|FlowControl|Gate true
    (:Exit
      (Transformation|SetRelativeRotation (Variables|Default|GetHand) (Math|Rotator|MakeRotator _roll (* (Math|Trig|Sin(Degrees) (* (- (Utilities|Time|GetTimeSeconds) (Variables|Default|GetStartTime)) 2e+02)) 5e+01) _yaw) false false))))

(fn ConstructionScript)