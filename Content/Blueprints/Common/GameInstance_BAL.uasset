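; Game instance for the two-player balance game that runs each client's rounds, from preparation through scoring.
; It maps spawn points by server-given indices, spawns falling objects on looping timers, and places both recipients, feeding positions into the rotating platform.
; It relays data to the server through PState, orienting positions and scores by IsServer.
; It also launches TCP matchmaking, shows widgets, and clears match data on network errors.
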(event Custom|Is%20Research%20Mode
  (bind _researchmode (Variables|Game|GetResearchMode))
  ;[1 1 1] Responsible for spawning and controlling game-related things over network on clients
  ;;[1 1 1] Send Server the research mode option
  (bind _aspstate (Utilities|Casting|CastToPState (Variables|/Script/Engine.Controller|GetPlayerState (Game|GetPlayerController 0)))
    (:then
      (Development|PrintText (Utilities|Text|FormatText "Client options on gi {0}" (Utilities|Text|ToText(Boolean) _researchmode)) false false "(R=1.000000,G=0.000000,B=0.260066,A=1.000000)" 5e+01)
      (Default|IsResearchModeResponse _aspstate _researchmode))
    (:CastFailed
      (Development|PrintString "cast failed"))))

(event Custom|Spawn%20Recipient
  (params (Location :type Vector))
  ;[1 1 1] Responsible for spawning and controlling game-related things over network on clients
  ;;[1 1 1] Spawn my player recipient  and Curtain
  (Variables|Game|SetPlayerPosition "NewEnumerator2")
  (Game|SpawnActorfromClass "/Game/Blueprints/Multiplayer/Balanca_Recipient.Balanca_Recipient_C" (Math|Transform|MakeTransform Location "0,90.000000, 0" "-1.000000,1.000000,1.000000") "Undefined" 0 true 0)
  (Game|SpawnActorfromClass "/Game/Blueprints/Common/Curtain.Curtain_C" (Math|Transform|MakeTransform (Variables|ActorLocations|Getlocation%20curtain) "0,0.000000, 0") "AlwaysSpawn" 0 0))

(event Custom|On%20PreParation%20Start
  (params (Spawn%20Index%201 :type Integer) (Spawn%20Index%202 :type Integer) (Spawn%20Index%203 :type Integer) (Spawn%20Index%204 :type Integer))
  ;[1 1 1] Responsible for spawning and controlling game-related things over network on clients
  ;;[1 1 1] Preparation Start configuration
  (Utilities|FlowControl|Sequence
    (:then_0
      (Variables|Game|SetRound%20State "NewEnumerator0")
      (Variables|GameSpawn|SetSpawn%20Index%201 Spawn%20Index%201)
      (Variables|GameSpawn|SetSpawn%20Index%202 Spawn%20Index%202)
      (Variables|GameSpawn|SetSpawn%20Index%203 Spawn%20Index%203)
      (Variables|GameSpawn|SetSpawn%20Index%204 Spawn%20Index%204)
      (bind _outactors (Actor|GetAllActorswithTag "SpawnTargetPoint"))
      (for _array_element _outactors
        ;;;[1 1 1] Storing spawn points
        (bind _astarget_point (Utilities|Casting|CastToTargetPoint _array_element))
        (switch string (Utilities|GetDisplayName _astarget_point)
          (:TargetPoint1
            (Utilities|Array|SetArrayElem (Variables|Game|GetSpawn%20Points) (Variables|GameSpawn|GetSpawn%20Index%201) _astarget_point))
          (:TargetPoint2
            (Utilities|Array|SetArrayElem (Variables|Game|GetSpawn%20Points) (Variables|GameSpawn|GetSpawn%20Index%202) _astarget_point))
          (:TargetPoint3
            (Utilities|Array|SetArrayElem (Variables|Game|GetSpawn%20Points) (Variables|GameSpawn|GetSpawn%20Index%203) _astarget_point))
          (:TargetPoint4
            (Utilities|Array|SetArrayElem (Variables|Game|GetSpawn%20Points) (Variables|GameSpawn|GetSpawn%20Index%204) _astarget_point)))))
    (:then_1
      (Utilities|IsValid (Variables|Game|GetW_GameStart)
        (:Is%20Valid
          (Widget|SetVisibility (Variables|Game|GetW_GameStart) "Visible")
          (Utilities|FlowControl|Delay 3.0)
          (Widget|SetVisibility (Variables|Game|GetW_GameStart) "Hidden"))
        (:Is%20Not%20Valid
          (bind _returnvalue (UserInterface|CreateWidget "/Game/HUD/W_GameStartWarning.W_GameStartWarning_C"))
          (bind _output_get (Variables|Game|SetW_GameStart _returnvalue))
          (UserInterface|Viewport|AddtoViewport _output_get 5)
          (Utilities|FlowControl|Delay 3.0)
          (Widget|SetVisibility _output_get "Hidden"))))))

(event Custom|Update%20Player%202%20Recipient
  (params (Recipient%20New%20Position :type Integer))
  ;[1 1 1] Responsible for spawning and controlling game-related things over network on clients
  ;;[1 1 1] Recieving other player's recipient position and spawn it
  (bind _returnvalue (Game|SpawnActorfromClass "/Game/Blueprints/Multiplayer/Balanca_Recipient.Balanca_Recipient_C" (Utilities|Select :Index Recipient%20New%20Position :Option%200 (Math|Transform|MakeTransform (Variables|ActorLocations|GetNo%20Coop%20Position) "0,90.000000, 0" "1,1.000000,1.000000") :Option%201 (Math|Transform|MakeTransform (Variables|ActorLocations|GetCoop%20Position) "0.000000,90.000000,0.000000" "1.000000,1.000000,1.000000") :Option%202 (Math|Transform|MakeTransform (Variables|ActorLocations|GetNeutral%20Second%20Player%20Location) "0,90.000000, 0" "1,1.000000,1.000000")) "Undefined" 0 false 0))
  (bind _output_get (Variables|Multiplayer|SetOther%20Recipient%20Final%20Position Recipient%20New%20Position))
  (Variables|Actors|SetSecondRecipient _returnvalue)
  (if (== _output_get 1)
    (Transformation|AttachActorToActor _returnvalue (Variables|Actors|GetRotatingPlataform) "None" "KeepWorld" "KeepWorld" "KeepWorld" true)
    (Default|CallOtherplayerRecipientDone _output_get)
    (else
      (Default|CallOtherplayerRecipientDone (Variables|Multiplayer|GetOther%20Recipient%20Final%20Position)))))

(event Custom|Receive%20Play%20Again%20Message
  (params (Msg :type Integer))
  ;[1 1 1] Responsible for spawning and controlling game-related things over network on clients
  (Default|CallPlayAgainMessageDispatcher Msg))

(event Custom|On%20PreParation%20Spawn
  (params (Spawn%20Interval%20A :type Float%20%28single-precision%29) (Spawn%20Interval%20B :type Float%20%28single-precision%29) (Quantity%20A1 :type Integer) (Quantity%20B1 :type Integer) (Round%20Timer :type Float%20%28single-precision%29))
  ;[1 1 1] Responsible for spawning and controlling game-related things over network on clients
  ;;[1 1 1] Preparation phase
  (Variables|SERVER|SetSpawn%20Interval%20A Spawn%20Interval%20A)
  (Variables|SERVER|SetSpawn%20Interval%20B Spawn%20Interval%20B)
  (Variables|SERVER|SetRound%20Timer Round%20Timer)
  (CallFunction|SpawnFallingObjects Quantity%20A1 Quantity%20B1))

(event Custom|Spawn%20A%20Objects
  ;[1 1 1] Responsible for spawning and controlling game-related things over network on clients
  ;;[1 1 1] Spawning falling objects
  (if (== (Variables|GameSpawn|GetQuantity%20A1) (Variables|SERVER|GetNumber%20A%20Spawned))
    (Utilities|Time|ClearandInvalidateTimerbyHandle (stale Custom|Spawn%20Falling%20Objects _returnvalue))
    (else
      (Math|Integer|IncrementInt (Variables|SERVER|GetNumber%20A%20Spawned)
        (:%20%20
          (Game|SpawnActorfromClass "/Game/Blueprints/Multiplayer/Balanca_FallingObject.Balanca_FallingObject_C" (Math|Conversions|ToTransform(Vector) (Transformation|GetActorLocation (Utilities|Array|Get(acopy) (Variables|Game|GetSpawn%20Points) (Variables|GameSpawn|GetSpawn%20Index%201)))) "Undefined" (Game|Player|GetPlayerPawn 0) 0)
          (Game|SpawnActorfromClass "/Game/Blueprints/Multiplayer/Balanca_FallingObject.Balanca_FallingObject_C" (Math|Conversions|ToTransform(Vector) (Variables|ActorLocations|GetA2%20Location)) "Undefined" 0 0))))))

(event Custom|Spawn%20B%20Objects
  ;[1 1 1] Responsible for spawning and controlling game-related things over network on clients
  ;;[1 1 1] Spawning falling objects
  (if (== (Variables|GameSpawn|GetQuantity%20B1) (Variables|SERVER|GetNumber%20B%20Spawned))
    (Utilities|Time|ClearandInvalidateTimerbyHandle (stale Custom|Spawn%20Falling%20Objects _returnvalue_2))
    (else
      (Math|Integer|IncrementInt (Variables|SERVER|GetNumber%20B%20Spawned)
        (:%20%20
          (Game|SpawnActorfromClass "/Game/Blueprints/Multiplayer/Balanca_FallingObject.Balanca_FallingObject_C" (Math|Conversions|ToTransform(Vector) (Transformation|GetActorLocation (Utilities|Array|Get(acopy) (Variables|Game|GetSpawn%20Points) (Variables|GameSpawn|GetSpawn%20Index%202)))) "Undefined" 0 0)
          (Game|SpawnActorfromClass "/Game/Blueprints/Multiplayer/Balanca_FallingObject.Balanca_FallingObject_C" (Math|Conversions|ToTransform(Vector) (Variables|ActorLocations|GetB2%20Location)) "Undefined" 0 0))))))

(event Custom|Send%20Player%20Information
  ;[1 1 1] Responsible for spawning and controlling game-related things over network on clients
  ;;[0.5151 1 0.01036] Send To Host the Player Data
  (bind _aspstate (Utilities|Casting|CastToPState (Variables|/Script/Engine.Controller|GetPlayerState (Game|GetPlayerController 0))))
  (Default|SendPlayerDatatoServer _aspstate (Variables|Data|GetPlayerData)))

(event Custom|Spawn%20Quantities
  (params (Quantity%20A1 :type Integer) (Quantity%20B1 :type Integer) (Quantity%20A2 :type Integer) (Quantity%20B2 :type Integer))
  ;[1 1 1] Responsible for spawning and controlling game-related things over network on clients
  ;;[1 1 1] Preparation Start configuration
  ;;;[1 1 1] Store the quantities of falling objects pre defined on server
  (Variables|GameSpawn|SetQuantity%20A1 Quantity%20A1)
  (Variables|GameSpawn|SetQuantity%20B1 Quantity%20B1)
  (Variables|GameSpawn|SetQuantity%20A2 Quantity%20A2)
  (Variables|GameSpawn|SetQuantity%20B2 Quantity%20B2))

(event Custom|Add%20Score
  (params (P1Score :type Integer) (P2Score :type Integer) (RoundPoints :type Integer))
  ;[1 0 0] Updates  own and other player scores
  (Variables|Multiplayer|SetRoundPoints RoundPoints)
  (if (Networking|IsServer)
    (Variables|Multiplayer|SetP1RoundScore P1Score)
    (Variables|Multiplayer|SetP2RoundScore P2Score)
    (else
      (Variables|Multiplayer|SetP2RoundScore P1Score)
      (Variables|Multiplayer|SetP1RoundScore P2Score)))
  (if (and (Utilities|IsValid (Variables|Actors|GetScoreActor1)) (Utilities|IsValid (Variables|Actors|GetScoreActor2)))
    _
    (else
      (CallFunction|GetScoreActors)))
  (Default|SetPlayerScore (Variables|Actors|GetScoreActor1))
  (Default|SetPlayerScore (Variables|Actors|GetScoreActor2)))

(event Custom|Spawn%20Falling%20Objects
  (params (Quantity%20A1 :type Integer) (Quantity%20B1 :type Integer))
  ;[1 1 1] Responsible for spawning and controlling game-related things over network on clients
  ;;[1 1 1] Spawning falling objects
  (bind _output_get (Variables|GameSpawn|SetQuantity%20A1 Quantity%20A1))
  (Variables|GameSpawn|SetQuantity%20A2 _output_get)
  (bind _output_get_2 (Variables|GameSpawn|SetQuantity%20B1 Quantity%20B1))
  (Variables|GameSpawn|SetQuantity%20B2 _output_get_2)
  (CallFunction|SpawnAObjects)
  (CallFunction|SpawnBObjects)
  (bind _returnvalue (Utilities|Time|SetTimerbyEvent (delegate Custom|Spawn%20A%20Objects) (Variables|SERVER|GetSpawn%20Interval%20A) true))
  (bind _returnvalue_2 (Utilities|Time|SetTimerbyEvent (delegate Custom|Spawn%20B%20Objects) (Variables|SERVER|GetSpawn%20Interval%20B) true)))

(event Custom|GetRotatingPlataform
  ;[1 1 1] Responsible for spawning and controlling game-related things over network on clients
  ;;[1 0.1694 0] Finding rotating plataform reference on post login
  (bind _outactors (Actor|GetAllActorsOfClass "/Game/Blueprints/Common/Balanca_RotatingPlataform.Balanca_RotatingPlataform_C"))
  (Variables|Actors|SetRotatingPlataform (Utilities|Array|Get(acopy) _outactors)))

(event Custom|Clear%20Info
  ;[1 1 1] Responsible for spawning and controlling game-related things over network on clients
  ;;[1 1 1] Clears the informations from last match
  (Variables|Data|SetMatchData "")
  (Variables|Game|SetMultiplayer false)
  (Variables|Data|SetPlayerData "")
  (Variables|Multiplayer|SetP1TotalScore 0)
  (Variables|Multiplayer|SetP2TotalScore 0)
  (Utilities|Array|Clear (Variables|Data|GetRoundData))
  (Variables|Data|SetScoreData "")
  (Variables|Multiplayer|SetP1RoundScore 0)
  (Variables|Multiplayer|SetP2RoundScore 0))

(event Custom|TCP
  ;[1 1 1] Responsible for spawning and controlling game-related things over network on clients
  ;;[1 0 0.2031] Launch TCP function to connect to the server to find other player
  (Utilities|IsValid (Variables|MatchMaking|GetTCPActor)
    (:Is%20Valid
      (Class|TCPActor|Launch (Variables|MatchMaking|GetTCPActor)))
    (:Is%20Not%20Valid
      (bind _returnvalue (Game|SpawnActorfromClass "/Script/Balanca.TCPActor" (Math|Transform|MakeTransform "0, 0, 0") "Undefined" 0 0))
      (bind _output_get (Variables|MatchMaking|SetTCPActor _returnvalue))
      (Class|TCPActor|Launch _output_get))))

(event Custom|RotatePlataformWithPositions
  (params (ServerPos :type Integer) (ClientPos :type Integer))
  (bind _rotatingplataform (Variables|Actors|GetRotatingPlataform))
  ;[1 1 1] Responsible for spawning and controlling game-related things over network on clients
  ;;[1 1 1] Rotating plataform
  (if (Networking|IsServer)
    (Default|EvaluateRotation _rotatingplataform ServerPos ClientPos)
    (else
      (Default|EvaluateRotation _rotatingplataform ClientPos ServerPos))))

(event Custom|Play%20Again%20Message
  (params (Msg :type Integer))
  ;[1 1 1] Responsible for spawning and controlling game-related things over network on clients
  (bind _aspstate (Utilities|Casting|CastToPState (Variables|/Script/Engine.Controller|GetPlayerState (Game|GetPlayerController 0))))
  (Default|SendPlayAgainMessagePState _aspstate (Networking|IsServer) Msg))

(event Custom|Show%20Score%20Widget
  ;[1 1 1] Responsible for spawning and controlling game-related things over network on clients
  (bind _returnvalue (UserInterface|CreateWidget "/Game/HUD/Menu/W_ShowScore.W_ShowScore_C" (Game|GetPlayerController 0)))
  (UserInterface|Viewport|AddtoViewport _returnvalue 0))

(event Custom|Get%20Score%20Actors
  ;[1 1 1] Set The score actors for both client and host
  (bind _outactors (Actor|GetAllActorsOfClass "/Game/Blueprints/Common/ScoreHolder.ScoreHolder_C"))
  (for _array_element _outactors
    (if (Utilities|Enum|Equal(Enum) (Utilities|GetDisplayName _array_element) "FirstScoreHolder")
      (Variables|Actors|SetScoreActor1 _array_element)
      (else
        (Variables|Actors|SetScoreActor2 _array_element)))))

(event Custom|Preparation%20%20Over%20Event
  ;[1 1 1] Responsible for spawning and controlling game-related things over network on clients
  ;;[1 0.0828 0.1126] Preparation over caller
  (Variables|Game|SetRound%20State "NewEnumerator1")
  (Default|CallPreparationOver))

(event Custom|Round%20Over
  ;[0.4187 1 0.4793] Event the happens when a round end
  (Variables|SERVER|SetNumber%20B%20Spawned 0)
  (Variables|SERVER|SetNumber%20A%20Spawned 0)
  (Variables|Multiplayer|SetRecipient%20Final%20Position -1)
  (Variables|Multiplayer|SetOther%20Recipient%20Final%20Position -1)
  (Default|CallRoundOver))

(event Custom|Clear%20Viewport
  ;[1 1 1] Responsible for spawning and controlling game-related things over network on clients
  (Default|CallClearViewportDispatcher))

(event Custom|Send%20Position%20to%20server
  ;[1 1 1] Responsible for spawning and controlling game-related things over network on clients
  ;;[1 1 1] Sending my recipient position to server
  (bind _aspstate (Utilities|Casting|CastToPState (Variables|/Script/Engine.Controller|GetPlayerState (Game|GetPlayerController 0))))
  (Default|ServerSendInfo _aspstate (Variables|Multiplayer|GetRecipient%20Final%20Position) (Networking|IsServer)))

(event EventHandleNetworkError
  (params (FailureType :type ENetworkFailure%20Enum :default "NetDriverAlreadyExists") (bIsServer :type Boolean))
  ;[1 0.2499 0.5686] Clear Info Whenever A Network Erro Happens
  (switch Utilities|FlowControl|Switch|SwitchonENetworkFailure FailureType
    (:ConnectionLost
      (CallFunction|ClearInfo))
    (:ConnectionTimeout
      (CallFunction|ClearInfo :!label _label))
    (:FailureReceived
      (goto _label))
    (:PendingConnectionFailure
      (goto _label)))
  (if bIsServer
    _
    (else
      _))
  (bind _returnvalue (UserInterface|CreateWidget "/Game/HUD/Menu/W_MenuMessages.W_MenuMessages_C"))
  (UserInterface|Viewport|AddtoViewport _returnvalue 0)
  (Rendering|Components|TextRender|SetText (Variables|/Game/HUD/Menu/W_MenuMessages.W_MenuMessages_C|GetTxt_MenuMessages _returnvalue) (Utilities|Select :Index FailureType :NetDriverAlreadyExists "" :NetDriverCreateFailure "" :NetDriverListenFailure "" :ConnectionLost "Desconectado" :ConnectionTimeout "Conexão Timeout" :FailureReceived "Falha" :OutdatedClient "Atualize o seu jogo" :OutdatedServer "" :PendingConnectionFailure "" :NetGuidMismatch "" :NetChecksumMismatch "")))