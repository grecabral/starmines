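; Rotating balance platform that tips left or right based on two players' recipient positions.
; Evaluaterotation picks a direction for unbalanced position pairs, runs a roll timeline that ends by opening one side, and disables the first attached recipient's tagged collision boxes.
; BeginPlay binds an empty preparation-over handler under Balanca_GameMode, otherwise binds the GameInstance round-over event to restore rotations and side collision.
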(event Custom|RotateForDirection
  (params (Direction :type Integer))
  (bind _right_plat (Variables|Default|GetRight%20Plat))
  (bind _left_part (Variables|Default|GetLeft%20Part))
  (bind _returnvalue (Transformation|GetWorldRotation _right_plat))
  (bind _returnvalue_2 (Transformation|GetWorldRotation _left_part))
  (bind (_roll _pitch _yaw) (Math|Rotator|BreakRotator _returnvalue))
  (bind (_roll_2 _pitch_2 _yaw_2) (Math|Rotator|BreakRotator _returnvalue_2))
  ;[1 1 1] Rotation
  (bind _rotation (Timeline|Rotation PlayFromStart)
    (:Update
      (Transformation|SetActorRotation (Math|Rotator|MakeRotator (Utilities|Select :Index Direction :Option%200 _rotation :Option%201 (* _rotation -1.0)) 0.0 0.0)))
    (:Finished
      (Collision|SetCollisionEnabled (Utilities|Select :Index Direction :Option%200 (Variables|Default|GetRBox) :Option%201 (Variables|Default|GetLBox)) "NoCollision")
      (if (== Direction 0)
        (Transformation|SetWorldRotation _right_plat (Math|Rotator|MakeRotator _roll 9e+01 _yaw) false false)
        (else
          (Transformation|SetWorldRotation _left_part (Math|Rotator|MakeRotator _roll_2 -9e+01 _yaw_2) false false))))))

(event Custom|RemoveCollisionFromRecipient
  (bind _outactors (Actor|GetAttachedActors))
  (bind _item (Utilities|Array|Get(acopy) _outactors))
  ;[1 1 1] Removing collision from rotated recipients
  (bind _asbalanca_recipient (Utilities|Casting|CastToBalanca_Recipient _item)
    (:then
      (for _array_element (Actor|GetComponentsbyTag _asbalanca_recipient "/Script/Engine.BoxComponent" "Collision")
        (Collision|SetCollisionEnabled _array_element "NoCollision")))
    (:CastFailed
      (bind _asbalanca_recipient_sp (Utilities|Casting|CastToBalanca_RecipientSP _item))
      (for _array_element_2 (Actor|GetComponentsbyTag _asbalanca_recipient_sp "/Script/Engine.BoxComponent" "Collision")
        (Collision|SetCollisionEnabled _array_element_2 "NoCollision")))))

(event Custom|Preparation%20Over%20Receiver
  ;[1 1 1] Begin Play
)

(event Custom|Reset%20Round
  ;[1 1 1] Reset Round
  (Transformation|SetActorRotation "0, 0, 0")
  (Collision|SetCollisionEnabled (Variables|Default|GetLBox) "QueryAndPhysics")
  (Collision|SetCollisionEnabled (Variables|Default|GetRBox) "QueryAndPhysics")
  (Transformation|SetWorldRotation (Variables|Default|GetRight%20Plat) "0,-90.000000, 0" false false))

(event Custom|Evaluate%20rotation
  (params (MyPosition :type Integer) (OtherPlayerPosition :type Integer))
  ;[1 1 1] Evaluating rotation based recipients' positions
  (if (not (or (or (and (== MyPosition 2) (== OtherPlayerPosition 0)) (and (== OtherPlayerPosition 2) (== MyPosition 0))) (or (and (== MyPosition 2) (== OtherPlayerPosition 2)) (or (and (== OtherPlayerPosition 1) (== MyPosition 1)) (and (== OtherPlayerPosition 0) (== MyPosition 0))))))
    (if (or (== OtherPlayerPosition 0) (== OtherPlayerPosition 2))
      (CallFunction|RotateforDirection 1)
      (Variables|Default|SetDirection 1)
      (else
        (CallFunction|RotateforDirection)
        (Variables|Default|SetDirection 0)))
    (CallFunction|RemoveCollisionfromRecipient)))

(event Custom|Round%20Over%20Receiver
  ;[1 1 1] Begin Play
  (CallFunction|ResetRound))

(event EventBeginPlay
  ;[1 1 1] Begin Play
  (bind _asbalanca_game_mode (Utilities|Casting|CastToBalanca_GameMode (Game|GetGameMode))
    (:then
      (EventDispatchers|BindEventtoPreparationOverDispatcher _asbalanca_game_mode (delegate Custom|Preparation%20Over%20Receiver)))
    (:CastFailed
      (bind _asgame_instance_bal (Utilities|Casting|CastToGameInstance_BAL (Game|GetGameInstance)))
      (EventDispatchers|BindEventtoRoundOver _asgame_instance_bal (delegate Custom|Round%20Over%20Receiver)))))

(fn ConstructionScript)