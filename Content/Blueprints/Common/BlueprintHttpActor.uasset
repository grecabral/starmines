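; Actor that checks for data files stored on the phone and sends them over HTTP.
; On BeginPlay it loads a widget, then polls on a looping timer, with an IsOpen flag gating each check.
; When data exists, it shows the sending indicator and main menu notification, then calls HttpCall if IsDone is set.
; When none remains, it hides both, with the menu notification toggled by alpha through the Menu_GameMode HUD.
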(event Custom|Check%20For%20Data
  ;[1 0.02672 0.1164] Http Actor is going to try to check for data files stored into the phone and then try to send them over http request
  (if (Variables|Default|GetisOpen)
    (Variables|Default|SetisOpen false)
    (if (not (Widget|IsVisible (Variables|Default|GetSendingFiles)))
      (Widget|SetVisibility (Variables|Default|GetSendingFiles) "Visible"))
    (bind (_data _isempty) (CallFunction|GetDataFiles))
    (if (not _isempty)
      (Utilities|ShowNotificationonMainMenu 1.0
        (:On%20Main%20Menu
          _)
        (:Not%20On%20Main%20Menu
          _))
      (if (Variables|Default|GetisDone)
        (Class|HttpActor|HttpCall _data)
        (Variables|Default|SetisOpen true)
        (else
          (Variables|Default|SetisOpen true)))
      (else
        (Widget|SetVisibility (Variables|Default|GetSendingFiles) "Hidden")
        (Utilities|ShowNotificationonMainMenu 0.0
          (:On%20Main%20Menu
            _)
          (:Not%20On%20Main%20Menu
            _))
        (Variables|Default|SetisOpen true)))))

(event EventBeginPlay
  ;[1 0.02672 0.1164] Http Actor is going to try to check for data files stored into the phone and then try to send them over http request
  (Class|HttpActor|LoadWidget)
  (Utilities|Time|SetTimerbyEvent (delegate Custom|Check%20For%20Data) 2.0 true))

(fn ConstructionScript)

(fn GetDataFiles
  (bind _returnvalue (Class|SaveandLoadFiles|LoadDatatoString))
  (return _returnvalue (== (Utilities|Array|Length _returnvalue) 0)))