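; Falling candy for the Balanca game that bounces along parabolic arcs and is destroyed when the round ends.
; BounceTo picks a left or right Timeline by recipient position, reading Balanca_GameMode or, if that cast fails, GameInstance_BAL with Network timelines.
; Timelines teleport the actor, then re-enable sprite physics, adding a random sideways impulse unless the position is neutral.
; Hitting a recipient's bottom collider plays a one-time sound.
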(event Custom|BounceTo
  (params (left :type Boolean))
  ;[1 1 1] Allows the falling object to make a bounce trajectory
  (bind _asbalanca_game_mode (Utilities|Casting|CastToBalanca_GameMode (Game|GetGameMode))
    (:then
      (if left
        (if (== (Variables|/Game/Blueprints/Gamemodes/Balanca_GameMode.Balanca_GameMode_C|GetRecipient%201 _asbalanca_game_mode) 2)
          (bind _candylocation (Timeline|ParaboleLeftRecipientNeutral PlayFromStart)
            (:Update
              (Transformation|SetActorLocation _candylocation false true))
            (:Finished
              (Physics|SetSimulatePhysics (Variables|Default|GetPaperSprite) true)))
          (else
            (bind _candylocation_2 (Timeline|ParaboleLeft PlayFromStart)
              (:Update
                (Transformation|SetActorLocation _candylocation_2 false true))
              (:Finished
                (Physics|SetSimulatePhysics (Variables|Default|GetPaperSprite) true)
                (Physics|AddImpulse (Variables|Default|GetPaperSprite) (Utilities|Select :Index (Math|Random|RandomIntegerinRange 0 2) :Option%200 "0,-500.000000,0" :Option%201 "0,-420.000000,0" :Option%202 "0,-460.000000,0") "None" true)))))
        (elif (== (Variables|/Game/Blueprints/Gamemodes/Balanca_GameMode.Balanca_GameMode_C|GetRecipient%201 _asbalanca_game_mode) 2)
          (bind _candylocation_3 (Timeline|ParaboleRightRecipientNeutral PlayFromStart)
            (:Update
              (Transformation|SetActorLocation _candylocation_3 false true))
            (:Finished
              (Physics|SetSimulatePhysics (Variables|Default|GetPaperSprite) true)))
          (else
            (bind _candylocation_4 (Timeline|ParaboleRight PlayFromStart)
              (:Update
                (Transformation|SetActorLocation _candylocation_4 false true))
              (:Finished
                (Physics|SetSimulatePhysics (Variables|Default|GetPaperSprite) true)
                (Physics|AddImpulse (Variables|Default|GetPaperSprite) (Utilities|Select :Index (Math|Random|RandomIntegerinRange 0 2) :Option%200 "0,500.000000,0" :Option%201 "0,420.000000,0" :Option%202 "0,460.000000,0") "None" true)))))))
    (:CastFailed
      (bind _asgame_instance_bal (Utilities|Casting|CastToGameInstance_BAL (Game|GetGameInstance)))
      (if left
        (if (or (== (Variables|/Game/Blueprints/Common/GameInstance_BAL.GameInstance_BAL_C|GetRecipient%20Final%20Position _asgame_instance_bal) 2) (== (Variables|/Game/Blueprints/Common/GameInstance_BAL.GameInstance_BAL_C|GetOther%20Recipient%20Final%20Position _asgame_instance_bal) 2))
          (bind _candylocation_5 (Timeline|ParaboleLeftRecipientNeutralNetwork PlayFromStart)
            (:Update
              (Transformation|SetActorLocation _candylocation_5 false true))
            (:Finished
              (Physics|SetSimulatePhysics (Variables|Default|GetPaperSprite) true)))
          (else
            (bind _candylocation_6 (Timeline|ParaboleLeftNetwork PlayFromStart)
              (:Update
                (Transformation|SetActorLocation _candylocation_6 false true))
              (:Finished
                (Physics|SetSimulatePhysics (Variables|Default|GetPaperSprite) true)
                (Physics|AddImpulse (Variables|Default|GetPaperSprite) (Utilities|Select :Index (Math|Random|RandomIntegerinRange 0 2) :Option%200 "0,-500.000000,0" :Option%201 "0,-420.000000,0" :Option%202 "0,-460.000000,0") "None" true)))))
        (elif (or (== (Variables|/Game/Blueprints/Common/GameInstance_BAL.GameInstance_BAL_C|GetRecipient%20Final%20Position _asgame_instance_bal) 2) (== (Variables|/Game/Blueprints/Common/GameInstance_BAL.GameInstance_BAL_C|GetOther%20Recipient%20Final%20Position _asgame_instance_bal) 2))
          (bind _candylocation_7 (Timeline|ParaboleRightRecipientNeutralNetwork PlayFromStart)
            (:Update
              (Transformation|SetActorLocation _candylocation_7 false true))
            (:Finished
              (Physics|SetSimulatePhysics (Variables|Default|GetPaperSprite) true)))
          (else
            (bind _candylocation_8 (Timeline|ParaboleRightNetwork PlayFromStart)
              (:Update
                (Transformation|SetActorLocation _candylocation_8 false true))
              (:Finished
                (Physics|SetSimulatePhysics (Variables|Default|GetPaperSprite) true)
                (Physics|AddImpulse (Variables|Default|GetPaperSprite) (Utilities|Select :Index (Math|Random|RandomIntegerinRange 0 2) :Option%200 "0,500.000000,0.000000" :Option%201 "0.000000,420.000000,0.000000" :Option%202 "0.000000,460.000000,0") "None" true)))))))))

(event Custom|Round%20Over%20Receiver
  (CallFunction|ResetRound))

(event Custom|Reset%20Round
  (Actor|DestroyActor))

(event Collision|EventHit
  (params (MyComp :type Primitive%20Component%20Object%20Reference) (Other :type Actor%20Object%20Reference) (OtherComp :type Primitive%20Component%20Object%20Reference) (bSelfMoved :type Boolean) (HitLocation :type Vector :default "0, 0, 0") (HitNormal :type Vector :default "0, 0, 0") (NormalImpulse :type Vector :default "0, 0, 0") (Hit :type Hit%20Result%20Structure%20%28by%20ref%29))
  (bind _asbalanca_recipient (Utilities|Casting|CastToBalanca_Recipient Other)
    (:then
      (if (== (Variables|/Game/Blueprints/Multiplayer/Balanca_Recipient.Balanca_Recipient_C|GetBottomCollider _asbalanca_recipient) OtherComp)
        (Utilities|FlowControl|DoOnce false
          (:Completed
            (Audio|PlaySound2D "/Game/Assets/Sounds/3GS_HitLow.3GS_HitLow")))))
    (:CastFailed
      (bind _asbalanca_recipient_sp (Utilities|Casting|CastToBalanca_RecipientSP Other))
      (if (== OtherComp (Variables|/Game/Blueprints/SinglePlayer/Balanca_RecipientSP.Balanca_RecipientSP_C|GetBottomCollider _asbalanca_recipient_sp))
        (Utilities|FlowControl|DoOnce false
          (:Completed
            (Audio|PlaySound2D "/Game/Assets/Sounds/3GS_HitLow.3GS_HitLow")))))))

(event EventBeginPlay
  (bind _asgame_instance_bal (Utilities|Casting|CastToGameInstance_BAL (Game|GetGameInstance)))
  (EventDispatchers|BindEventtoRoundOver _asgame_instance_bal (delegate Custom|Round%20Over%20Receiver)))

(fn ConstructionScript)