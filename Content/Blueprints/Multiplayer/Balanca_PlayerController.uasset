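; Player controller for the Balanca multiplayer content that lets touch input drag Balanca_Recipient actors.
; A press traces under the first finger for a recipient object, stores it and opens a gate, or clears it and closes the gate.
; While open, Tick and touch-move events move the recipient to the Camera-channel hit point.
; Release passes the finger and deprojected world location to the recipient, then closes the gate.
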(event EventTick
  (params (DeltaSeconds :type Float%20%28single-precision%29))
  (bind (_hitresult _returnvalue) (Class|PlayerController|GetHitResultUnderFingerbyChannel "Touch1" "TraceTypeQuery2" true))
  ;[1 1 1] Move Recipient on touch events
  (Utilities|FlowControl|Gate true
    (:Exit
      (if _returnvalue
        (Default|MovetoPosition (Variables|Default|GetRecipient) (.Location (Collision|BreakHitResult _hitresult)))))))

(event Input|TouchEvents|InputTouch
  (params (Location :type Vector) (FingerIndex :type ETouchIndex%20Enum))
  (bind (_hitresult _returnvalue) (Class|PlayerController|GetHitResultUnderFingerbyChannel "Touch1" "TraceTypeQuery2" true))
  (bind (_x _y) (Math|Vector|BreakVector Location))
  (bind _array (Utilities|Array|MakeArray "ObjectTypeQuery8"))
  (bind (_hitresult_2 _returnvalue_2) (Class|PlayerController|GetHitResultUnderFingerforObjects "Touch1" _array true))
  ;[1 1 1] Move Recipient on touch events
  (:Pressed
    (if _returnvalue_2
      (bind _asbalanca_recipient (Utilities|Casting|CastToBalanca_Recipient (.HitActor (Collision|BreakHitResult _hitresult_2))))
      (Variables|Default|SetRecipient _asbalanca_recipient)
      (goto _label Open)
      (else
        (Variables|Default|SetRecipient 0)
        (goto _label Close))))
  (:Released
    (Utilities|IsValid (Variables|Default|GetRecipient)
      (:Is%20Valid
        (Default|ReleaseTouch (Variables|Default|GetRecipient) FingerIndex (.WorldLocation (Class|PlayerController|DeprojectScreenPositiontoWorld _x _y)))
        (goto _label Close))))
  (:Moved
    (Utilities|FlowControl|Gate true :!label _label
      (:Exit
        (if _returnvalue
          (Default|MovetoPosition (Variables|Default|GetRecipient) (.Location (Collision|BreakHitResult _hitresult))))))))

(fn ConstructionScript)