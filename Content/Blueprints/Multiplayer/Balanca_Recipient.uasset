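; Movable recipient for the multiplayer Balanca game, dragged by touch along Y between two tagged snapping points, with a hand indicator when controlled.
; Release snaps it to the nearer point and records the position in GameInstance_BAL, unless player state dictates a third value.
; GameInstance events drive the round: preparation end snaps it, sends the controlled position to the server and attaches it to the rotating platform at position 1; round end destroys it.
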(event Custom|Move%20to%20position
  (params (TouchPosition :type Vector))
  (bind _returnvalue (Transformation|GetActorLocation))
  (bind _snappingpoints (Variables|Default|GetSnappingPoints))
  (bind (_x _y) (Math|Vector|BreakVector _returnvalue))
  ;[1 1 1] Recipient Movement
  ;;[1 1 1] Moving on touch hold
  (CallFunction|DeleteActorIndicator)
  (bind _asgame_instance_bal (Utilities|Casting|CastToGameInstance_BAL (Game|GetGameInstance)))
  (Variables|/Game/Blueprints/Common/GameInstance_BAL.GameInstance_BAL_C|SetPlayerPosition _asgame_instance_bal "NewEnumerator0")
  (bind _game_state (CallFunction|GetGameinProgress))
  (if _game_state
    (Transformation|SetActorLocation (Math|Vector|MakeVector _x (Math|Interpolation|FInterpTo _y (Math|Float|Clamp(Float) (.Y (Math|Vector|BreakVector TouchPosition)) (.Y (Math|Vector|BreakVector (Transformation|GetActorLocation (Utilities|Array|Get(acopy) _snappingpoints)))) (.Y (Math|Vector|BreakVector (Transformation|GetActorLocation (Utilities|Array|Get(acopy) _snappingpoints 1))))) (Utilities|Time|GetWorldDeltaSeconds) 3.0) -2e+02) true false)))

(event Custom|Show%20Hand%20Indicator
  ;[1 1 1] Spanws Actor Indicator to show the player where to move the recipient
  (bind _returnvalue (Game|SpawnActorfromClass "/Game/Blueprints/Common/HandActor.HandActor_C" (Math|Transform|MakeTransform (Transformation|GetWorldLocation (Variables|Default|GetBillboard)) "0,0.000000, 0") "Undefined" 0 0))
  (Variables|Default|SetHandIndicatorActor _returnvalue))

(event Custom|Preparation%20Over%20Delegate
  ;[1 1 1] Configuration code
  (CallFunction|PreparationOver))

(event Custom|Preparation%20Over
  (bind _snappingpoints (Variables|Default|GetSnappingPoints))
  ;[1 1 1] Recipient Movement
  (Utilities|FlowControl|Sequence
    (:then_0
      ;;[1 1 1] Snapping on Round Over
      (bind _snappedposition (CallFunction|SnapRecipient (.Y (Math|Vector|BreakVector (Transformation|GetActorLocation (Utilities|Array|Get(acopy) _snappingpoints)))) (.Y (Math|Vector|BreakVector (Transformation|GetActorLocation (Utilities|Array|Get(acopy) _snappingpoints 1)))) (.Location (Collision|BreakHitResult (.HitResult (Game|Player|GetHitResultUnderCursorbyChannel (Game|GetPlayerController 0) "TraceTypeQuery1" true))))))
      (Variables|Default|SetSnappedPosition _snappedposition)
      (bind _asgame_instance_bal (Utilities|Casting|CastToGameInstance_BAL (Game|GetGameInstance)))
      (if (Variables|Default|GetisControlled)
        (Default|SendPositiontoServer _asgame_instance_bal)))
    (:then_1
      ;;[1 1 1] Attaching to rotating plataform when on it
      (if (== (Variables|Default|GetSnappedPosition) 1)
        (bind _outactors (Actor|GetAllActorsOfClass "/Game/Blueprints/Common/Balanca_RotatingPlataform.Balanca_RotatingPlataform_C"))
        (Transformation|AttachActorToActor (Utilities|Array|Get(acopy) _outactors) "None" "KeepWorld" "KeepWorld" "KeepWorld" true)))))

(event Custom|Delete%20Actor%20Indicator
  (bind _handindicatoractor (Variables|Default|GetHandIndicatorActor))
  ;[1 1 1] Deletes The Actor indicator
  (Utilities|IsValid _handindicatoractor
    (:Is%20Valid
      (Actor|DestroyActor _handindicatoractor))))

(event Custom|Round%20Over%20Receiver
  ;[1 1 1] Configuration code
  (CallFunction|RoundReset))

(event Custom|Release%20Touch
  (params (Finger%20Index :type ETouchIndex%20Enum) (Release%20Location :type Vector))
  (bind _snappingpoints (Variables|Default|GetSnappingPoints))
  ;[1 1 1] Recipient Movement
  ;;[1 1 1] Snapping on release
  (bind _game_state (CallFunction|GetGameinProgress))
  (if _game_state
    (bind _snappedposition (CallFunction|SnapRecipient (.Y (Math|Vector|BreakVector (Transformation|GetActorLocation (Utilities|Array|Get(acopy) _snappingpoints)))) (.Y (Math|Vector|BreakVector (Transformation|GetActorLocation (Utilities|Array|Get(acopy) _snappingpoints 1)))) Release%20Location))
    (Variables|Default|SetSnappedPosition _snappedposition)))

(event Custom|Round%20Reset
  ;[1 1 1] Reset Round
  (CallFunction|DeleteActorIndicator)
  (Actor|DestroyActor))

(event EventBeginPlay
  (bind _snappingpoints (Variables|Default|GetSnappingPoints))
  ;[1 1 1] Configuration code
  (if (Variables|Default|GetisControlled)
    (CallFunction|ShowHandIndicator))
  (Utilities|FlowControl|Sequence
    (:then_0
      ;;[1 1 1] Setting Snapping points
      (bind _outactors (Actor|GetAllActorswithTag "SnappingTargetPoint"))
      (for _array_element _outactors
        (bind _astarget_point (Utilities|Casting|CastToTargetPoint _array_element))
        (switch string (Utilities|GetDisplayName _astarget_point)
          (:SnappingPoint1
            (Utilities|Array|SetArrayElem _snappingpoints 0 _astarget_point))
          (:SnappingPoint2
            (Utilities|Array|SetArrayElem _snappingpoints 1 _astarget_point))))
      (Variables|Default|SetSnappedPosition 0))
    (:then_1
      (bind _asgame_instance_bal (Utilities|Casting|CastToGameInstance_BAL (Game|GetGameInstance)))
      (if (Variables|Default|GetisControlled)
        (EventDispatchers|BindEventtoPreparationOver _asgame_instance_bal (delegate Custom|Preparation%20Over%20Delegate)))
      (EventDispatchers|BindEventtoRoundOver _asgame_instance_bal (delegate Custom|Round%20Over%20Receiver)))))

(fn ConstructionScript)

(fn GetGameinProgress
  (bind _asgame_instance_bal (Utilities|Casting|CastToGameInstance_BAL (Game|GetGameInstance))
    (:then
      (return (Utilities|Enum|Equal(Enum) (Variables|/Game/Blueprints/Common/GameInstance_BAL.GameInstance_BAL_C|GetRound%20State _asgame_instance_bal) "NewEnumerator0")))
    (:CastFailed
      (return false))))

(fn SnapRecipient
  (params (SnapPoint1Y :type Float%20%28single-precision%29) (SnapPoint2Y :type Float%20%28single-precision%29) (Mouse%20Input%20Location :type Vector))
  (bind _returnvalue (Transformation|GetActorLocation))
  (bind _y (Math|Vector|BreakVector Mouse%20Input%20Location))
  (bind (_x _y_2 _z) (Math|Vector|BreakVector _returnvalue))
  (bind _asgame_instance_bal (Utilities|Casting|CastToGameInstance_BAL (Game|GetGameInstance)))
  (if (Utilities|Enum|NotEqual(Enum) (Variables|/Game/Blueprints/Common/GameInstance_BAL.GameInstance_BAL_C|GetPlayerPosition _asgame_instance_bal) "NewEnumerator2")
    (if (< (Math|Float|Absolute(Float) (- _y SnapPoint1Y)) (Math|Float|Absolute(Float) (- _y SnapPoint2Y)))
      (Transformation|SetActorLocation (Math|Vector|MakeVector _x SnapPoint1Y _z) true false)
      (bind _asgame_instance_bal_2 (Utilities|Casting|CastToGameInstance_BAL (Game|GetGameInstance))
        (:then
          (bind _output_get (Variables|/Game/Blueprints/Common/GameInstance_BAL.GameInstance_BAL_C|SetRecipient%20Final%20Position _asgame_instance_bal_2 0)))
        (:CastFailed
          _))
      (return _output_get)
      (else
        (Transformation|SetActorLocation (Math|Vector|MakeVector _x SnapPoint2Y _z) true false)
        (bind _asgame_instance_bal_3 (Utilities|Casting|CastToGameInstance_BAL (Game|GetGameInstance))
          (:then
            (bind _output_get_2 (Variables|/Game/Blueprints/Common/GameInstance_BAL.GameInstance_BAL_C|SetRecipient%20Final%20Position _asgame_instance_bal_3 1)))
          (:CastFailed
            _))
        (return _output_get_2)))
    (else
      (bind _asgame_instance_bal_4 (Utilities|Casting|CastToGameInstance_BAL (Game|GetGameInstance))
        (:then
          (bind _output_get_3 (Variables|/Game/Blueprints/Common/GameInstance_BAL.GameInstance_BAL_C|SetRecipient%20Final%20Position _asgame_instance_bal_4 2)))
        (:CastFailed
          _))
      (return _output_get_3))))