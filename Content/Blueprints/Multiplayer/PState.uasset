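; Multiplayer player state for the Balanca game that acts as a messenger between the game instance and the game modes.
; Events for preparation, spawning, platform rotation, scores, round end and UI forward to GameInstance_BAL.
; Recipient position, play-again messages, player data and research-mode replies go to the network or lobby game mode.
; Each event is a thin cast-and-forward; only the player data request adds a non-server check.
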(event Custom|Preparation%20Match
  (params (Spawn%20Index%201 :type Integer) (Spawn%20Index%202 :type Integer) (Spawn%20Index%203 :type Integer) (Spawn%20Index%204 :type Integer) (Location :type Vector) (Spawn%20Interval%20A :type Float%20%28single-precision%29) (Spawn%20Interval%20B :type Float%20%28single-precision%29) (Quantity%20A1 :type Integer) (Quantity%20B1 :type Integer) (Round%20Timer :type Float%20%28single-precision%29))
  ;[1 1 1] Player state is our middle man on communications that transfer the info from the game instance to game mode
  ;;[1 1 1] Preparation match begin
  (bind _asgame_instance_bal (Utilities|Casting|CastToGameInstance_BAL (Game|GetGameInstance)))
  (Default|OnPreParationStart _asgame_instance_bal Spawn%20Index%201 Spawn%20Index%202 Spawn%20Index%203 Spawn%20Index%204)
  (Default|SpawnRecipient _asgame_instance_bal Location)
  (Default|OnPreParationSpawn _asgame_instance_bal Spawn%20Interval%20A Spawn%20Interval%20B Quantity%20A1 Quantity%20B1 Round%20Timer))

(event Custom|Preparation%20End
  ;[1 1 1] Player state is our middle man on communications that transfer the info from the game instance to game mode
  ;;[1 1 1] End of preparation phase
  (bind _asgame_instance_bal (Utilities|Casting|CastToGameInstance_BAL (Game|GetGameInstance)))
  (Default|PreparationOverEvent _asgame_instance_bal))

(event Custom|Round%20Over
  ;[1 1 1] Player state is our middle man on communications that transfer the info from the game instance to game mode
  ;;[1 1 1] Asking game instance to execute round over
  (bind _asgame_instance_bal (Utilities|Casting|CastToGameInstance_BAL (Game|GetGameInstance)))
  (Default|RoundOver _asgame_instance_bal))

(event Custom|Receive%20Play%20Again%20Message%20PState
  (params (Msg :type Integer))
  ;[1 1 1] Player state is our middle man on communications that transfer the info from the game instance to game mode
  ;;[1 1 1] Play Againg Messages Exchange
  (bind _asgame_instance_bal (Utilities|Casting|CastToGameInstance_BAL (Game|GetGameInstance)))
  (Default|ReceivePlayAgainMessage _asgame_instance_bal Msg))

(event Custom|GetRotatingPlataform
  ;[1 1 1] Player state is our middle man on communications that transfer the info from the game instance to game mode
  ;;[1 1 1] Asking game instance to set rotating plataform
  (bind _asgame_instance_bal (Utilities|Casting|CastToGameInstance_BAL (Game|GetGameInstance)))
  (Default|GetRotatingPlataform _asgame_instance_bal))

(event Custom|Is%20Research%20mode%20Response
  (params (Client%20Research%20Mode :type Boolean))
  ;[1 1 1] Server asking to client for research mode option
  (bind _asbalanca_game_mode_lobby (Utilities|Casting|CastToBalanca_GameMode_Lobby (Game|GetGameMode)))
  (Default|SetResearchModeNetwork _asbalanca_game_mode_lobby Client%20Research%20Mode))

(event Custom|RotatePlataformWithPositions
  (params (ServerPos :type Integer) (ClientPos :type Integer))
  ;[1 1 1] Player state is our middle man on communications that transfer the info from the game instance to game mode
  ;;[1 1 1] Rotates The Platform
  (bind _asgame_instance_bal (Utilities|Casting|CastToGameInstance_BAL (Game|GetGameInstance)))
  (Default|RotatePlataformwithPositions _asgame_instance_bal ServerPos ClientPos))

(event Custom|Server_Send%20Info
  (params (My%20Recipient%20Position :type Integer) (IsServer :type Boolean))
  ;[1 1 1] Player state is our middle man on communications that transfer the info from the game instance to game mode
  ;;[1 1 1] Sending other player's info to server
  (bind _asbalanca_game_mode_net_work (Utilities|Casting|CastToBalanca_GameMode_NetWork (Game|GetGameMode)))
  (Default|ReceiveClientUpdate _asbalanca_game_mode_net_work My%20Recipient%20Position IsServer))

(event Custom|Ask%20For%20Player%20For%20Data
  ;[1 1 1] Player state is our middle man on communications that transfer the info from the game instance to game mode
  ;;[1 0.7376 0.03484] Ask For Players For Their Datas
  (if (not (Networking|IsServer))
    (bind _asgame_instance_bal (Utilities|Casting|CastToGameInstance_BAL (Game|GetGameInstance)))
    (Default|SendPlayerInformation _asgame_instance_bal)))

(event Custom|Show%20Score%20To%20Player
  ;[1 1 1] Player state is our middle man on communications that transfer the info from the game instance to game mode
  (bind _asgame_instance_bal (Utilities|Casting|CastToGameInstance_BAL (Game|GetGameInstance)))
  (Default|ShowScoreWidget _asgame_instance_bal))

(event Custom|Send%20Play%20Again%20Message%20PState
  (params (Is%20Server :type Boolean) (Msg :type Integer))
  ;[1 1 1] Player state is our middle man on communications that transfer the info from the game instance to game mode
  ;;[1 1 1] Play Againg Messages Exchange
  (bind _asbalanca_game_mode_net_work (Utilities|Casting|CastToBalanca_GameMode_NetWork (Game|GetGameMode)))
  (Default|PlayAgainEvent _asbalanca_game_mode_net_work Is%20Server Msg))

(event Custom|Clear%20ViewPort%20Clients
  ;[1 1 1] Player state is our middle man on communications that transfer the info from the game instance to game mode
  (bind _asgame_instance_bal (Utilities|Casting|CastToGameInstance_BAL (Game|GetGameInstance)))
  (Default|ClearViewport _asgame_instance_bal))

(event Custom|Update%20Round%20Score
  (params (P1RoundScore :type Integer) (P2RoundScore :type Integer) (RoundPoints :type Integer))
  ;[1 1 1] Player state is our middle man on communications that transfer the info from the game instance to game mode
  ;;[1 1 1] Updat the players scores
  (bind _asgame_instance_bal (Utilities|Casting|CastToGameInstance_BAL (Game|GetGameInstance)))
  (Default|AddScore _asgame_instance_bal P1RoundScore P2RoundScore RoundPoints))

(event Custom|is%20Research%20mode
  ;[1 1 1] Server asking to client for research mode option
  (bind _asgame_instance_bal (Utilities|Casting|CastToGameInstance_BAL (Game|GetGameInstance)))
  (Default|IsResearchMode _asgame_instance_bal))

(event Custom|Set%20Player%20Scores%20on%20clients
  (params (ScoreData :type F%20Score%20Structure))
  (bind _asgame_instance_bal (Utilities|Casting|CastToGameInstance_BAL (Game|GetGameInstance)))
  (Variables|/Game/Blueprints/Common/GameInstance_BAL.GameInstance_BAL_C|SetScoreData _asgame_instance_bal ScoreData))

(event Custom|Send%20Player%20Data%20To%20Server
  (params (Player%20Data :type Player%20Data%20Structure))
  ;[1 1 1] Player state is our middle man on communications that transfer the info from the game instance to game mode
  ;;[0.9567 1 0.399] Send Client Data To The Host Server
  (bind _asbalanca_game_mode_net_work (Utilities|Casting|CastToBalanca_GameMode_NetWork (Game|GetGameMode)))
  (Default|SetSecondPlayerInformation _asbalanca_game_mode_net_work Player%20Data))

(event Custom|Update%20Player%202%20Recipient
  (params (Other%20Player%20Recipient%20pos :type Integer))
  ;[1 1 1] Player state is our middle man on communications that transfer the info from the game instance to game mode
  ;;[1 1 1] Updating other player's recipient position
  (bind _asgame_instance_bal (Utilities|Casting|CastToGameInstance_BAL (Game|GetGameInstance)))
  (Default|UpdatePlayer2Recipient _asgame_instance_bal Other%20Player%20Recipient%20pos))

(fn ConstructionScript)