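; Single-player falling object for the Balanca game that drops onto a rotating platform or into a recipient.
; During preparation a timeline drives its height over the game mode's preparation time; when preparation ends, sprite physics switches on.
; Hitting a recipient's bottom collider plays a sound and applies a random impulse.
; Hitting the platform replaces it with a Balanca_ParabolicObject, spawned and bounced toward a side based on platform direction.
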(event Custom|Preparation%20Over%20Receiver
  ;[1 1 1] Falling with calculated time to arrive at end point
  (CallFunction|PreparationOver))

(event Custom|Round%20Over%20Receiver
  ;[1 1 1] Falling with calculated time to arrive at end point
  (CallFunction|ResetRound))

(event Custom|Preparation%20Over
  ;[1 1 1] Round Over
  (Physics|SetSimulatePhysics (Variables|Default|GetPaperSprite) true))

(event Custom|Reset%20Round
  ;[1 1 1] Reset Round
  (Actor|DestroyActor))

(event EventBeginPlay
  (bind _returnvalue (Transformation|GetActorLocation))
  (bind (_x _y) (Math|Vector|BreakVector _returnvalue))
  ;[1 1 1] Falling with calculated time to arrive at end point
  (bind _asbalanca_game_mode (Utilities|Casting|CastToBalanca_GameMode (Game|GetGameMode)))
  (EventDispatchers|BindEventtoPreparationOverDispatcher _asbalanca_game_mode (delegate Custom|Preparation%20Over%20Receiver))
  (if (Utilities|Enum|Equal(Enum) (Variables|/Game/Blueprints/Gamemodes/Balanca_GameMode.Balanca_GameMode_C|GetRoundState _asbalanca_game_mode) "NewEnumerator0")
    (Components|Timeline|SetPlayRate (Variables|Default|GetFall_Timeline) (/ 1.0 (Variables|/Game/Blueprints/Gamemodes/Balanca_GameMode.Balanca_GameMode_C|GetPreparation%20Time _asbalanca_game_mode)))
    (bind _fall (Timeline|Fall_Timeline PlayFromStart)
      (:Update
        (Transformation|SetActorLocation (Math|Vector|MakeVector _x _y _fall) false false)))
    (else
      (CallFunction|PreparationOver)
      (Timeline|Fall_Timeline PlayFromStart))))

(event Collision|EventHit
  (params (MyComp :type Primitive%20Component%20Object%20Reference) (Other :type Actor%20Object%20Reference) (OtherComp :type Primitive%20Component%20Object%20Reference) (bSelfMoved :type Boolean) (HitLocation :type Vector) (HitNormal :type Vector :default "0, 0, 0") (NormalImpulse :type Vector :default "0, 0, 0") (Hit :type Hit%20Result%20Structure%20%28by%20ref%29))
  ;[1 1 1] Event hit the allows the falling objects to bounce to their respective recipient
  (bind _asbalanca_recipient_sp (Utilities|Casting|CastToBalanca_RecipientSP Other)
    (:then
      (if (== OtherComp (Variables|/Game/Blueprints/SinglePlayer/Balanca_RecipientSP.Balanca_RecipientSP_C|GetBottomCollider _asbalanca_recipient_sp))
        (Utilities|FlowControl|DoOnce false
          (:Completed
            (Audio|PlaySound2D "/Game/Assets/Sounds/3GS_HitLow.3GS_HitLow")
            (Physics|AddImpulse (Variables|Default|GetPaperSprite) (Utilities|Select :Index (Math|Random|RandomIntegerinRange 0 3) :Option%200 "0,50.000000,0" :Option%201 "0,-50.000000,0" :Option%202 "0,50.000000,25.000000" :Option%203 "0,-50.000000,-25.000000") "None" true)))))
    (:CastFailed
      (bind _asbalanca_rotating_plataform (Utilities|Casting|CastToBalanca_RotatingPlataform Other))
      (if (== (Variables|/Game/Blueprints/Common/Balanca_RotatingPlataform.Balanca_RotatingPlataform_C|GetDirection _asbalanca_rotating_plataform) 0)
        (Utilities|IsValid (Utilities|Array|Get(acopy) (Actor|GetComponentsbyTag _asbalanca_rotating_plataform "/Script/Engine.BoxComponent" "Side1"))
          (:Is%20Valid
            (Utilities|FlowControl|DoOnce false
              (:Completed
                (bind _returnvalue (Game|SpawnActorfromClass "/Game/Blueprints/Multiplayer/Balanca_ParabolicObject.Balanca_ParabolicObject_C" (Math|Transform|MakeTransform "420.000000,180.000000,121.000000") "Undefined" 0 0))
                (Default|Bounceto _returnvalue true)
                (Actor|DestroyActor)))))
        (elif (== (Variables|/Game/Blueprints/Common/Balanca_RotatingPlataform.Balanca_RotatingPlataform_C|GetDirection _asbalanca_rotating_plataform) 1)
          (Utilities|IsValid (Utilities|Array|Get(acopy) (Actor|GetComponentsbyTag _asbalanca_rotating_plataform "/Script/Engine.BoxComponent" "Side2"))
            (:Is%20Valid
              (bind _returnvalue_2 (Game|SpawnActorfromClass "/Game/Blueprints/Multiplayer/Balanca_ParabolicObject.Balanca_ParabolicObject_C" (Math|Transform|MakeTransform "420.000000,-180.000000,121.000000") "Undefined" 0 0))
              (Default|Bounceto _returnvalue_2 false)
              (Actor|DestroyActor))))))))

(fn ConstructionScript)