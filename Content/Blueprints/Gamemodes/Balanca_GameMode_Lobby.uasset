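; Lobby game mode for a two-player Balanca match that shows the match data widget and server-travels to the game map when ready.
; When a remote player logs in, a looping timer polls its PlayerState for the research mode option until SetResearchModeNetwork merges it into the GameInstance.
; Tick starts travel once Start is set, two players are present and that exchange completes.
; A remote logout before travel disables the widget and shows a player-left message.
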(event Custom|Get%20Client%20Research%20Option
  ;[1 0.1036 0] Waits for the client to send the research mode options
  (CallFunction|PSClientResearchOption))

(event Custom|PS%20Client%20Research%20Option
  ;[1 0.1036 0] Waits for the client to send the research mode options
  (bind _aspstate (Utilities|Casting|CastToPState (Variables|/Script/Engine.Controller|GetPlayerState (Variables|Controller|Get2ndPlayerController))))
  (Default|IsResearchMode _aspstate))

(event Custom|Set%20Research%20Mode%20Network
  (params (Client%20Research%20Mode :type Boolean))
  (bind _returnvalue (Game|GetGameInstance))
  ;[1 0.1036 0] Waits for the client to send the research mode options
  (Utilities|IsValid _returnvalue
    (:Is%20Valid
      (bind _asgame_instance_bal (Utilities|Casting|CastToGameInstance_BAL _returnvalue))
      (Variables|/Game/Blueprints/Common/GameInstance_BAL.GameInstance_BAL_C|SetResearchMode _asgame_instance_bal (or (Variables|/Game/Blueprints/Common/GameInstance_BAL.GameInstance_BAL_C|GetResearchMode _asgame_instance_bal) Client%20Research%20Mode))
      (Variables|StartControl|Setresearch%20mode%20completed true)
      (Utilities|Time|ClearandInvalidateTimerbyHandle (stale EventPostLogin _returnvalue)))))

(event EventBeginPlay
  ;[1 1 1] Adds widget to viewport
  (bind _returnvalue (UserInterface|CreateWidget "/Game/HUD/Menu/W_MatchData.W_MatchData_C"))
  (UserInterface|Viewport|AddtoViewport _returnvalue 0))

(event EventTick
  (params (DeltaSeconds :type Float%20%28single-precision%29))
  ;[1 1 1] Conditions to travel to game map
  (if (Math|Boolean|ANDBoolean (Variables|StartControl|GetStart) (== (Utilities|Array|Length (Variables|/Script/Engine.GameStateBase|GetPlayerArray (Game|GetGameState))) 2) (Variables|StartControl|Getresearch%20mode%20completed))
    (Variables|Default|SetisTravelling true)
    (Development|ExecuteConsoleCommand "servertravel Balanca_MapNetWork2")))

(event EventOnLogout
  (params (ExitingController :type Controller%20Object%20Reference))
  ;[1 1 1] Happens when the player exits
  (if (and (not (Pawn|IsLocalController ExitingController)) (not (Variables|Default|GetisTravelling)))
    (bind _returnvalue (UserInterface|CreateWidget "/Game/HUD/Menu/W_MenuMessages.W_MenuMessages_C"))
    (bind _foundwidgets (Widget|GetAllWidgetsOfClass "/Game/HUD/Menu/W_MatchData.W_MatchData_C" false))
    (Widget|SetIsEnabled (Utilities|Array|Get(acopy) _foundwidgets) false)
    (UserInterface|Viewport|AddtoViewport _returnvalue 0)
    (Rendering|Components|TextRender|SetText (Variables|/Game/HUD/Menu/W_MenuMessages.W_MenuMessages_C|GetTxt_MenuMessages _returnvalue) "Player 2 Saiu")))

(event EventPostLogin
  (params (NewPlayer :type Player%20Controller%20Object%20Reference))
  ;[1 0.1036 0] Waits for the client to send the research mode options
  (if (not (Pawn|IsLocalPlayerController NewPlayer))
    (Variables|Controller|Set2ndPlayerController NewPlayer)
    (bind _returnvalue (Utilities|Time|SetTimerbyEvent (delegate Custom|Get%20Client%20Research%20Option) 0.1 true))))

(fn ConstructionScript)