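; Server game mode for Balanca, a networked two-player cooperation game where recipient placement decides each player's points.
; Tick uses DoOnce gates to start once two players join, then to rotate platforms and score after both placements arrive.
; Match settings come from the GameInstance, and phases, timers and scores reach clients through each PState.
; Rounds repeat until the final score screen, with JSON saving in research mode and rematch support.
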(event Custom|On%20Preparation%20End%20BroadCast
  ;[1 1 1] Game owner logic (server side on networking)
  ;;[1 1 1] Preparation end and broadcast it to all clients
  (for _array_element (Variables|/Script/Engine.GameStateBase|GetPlayerArray (Game|GetGameState))
    (bind _aspstate (Utilities|Casting|CastToPState _array_element))
    (Default|PreparationEnd _aspstate)))

(event Custom|Set%20Round%20Score
  (bind _spawn_quantity_a1 (Variables|Spawn|GetSpawn%20Quantity%20A1))
  (bind _spawn_quantity_b1 (Variables|Spawn|GetSpawn%20Quantity%20B1))
  (bind _spawn_quantity_b1_2 (Variables|Spawn|GetSpawn%20Quantity%20B1))
  (bind _spawn_quantity_a1_2 (Variables|Spawn|GetSpawn%20Quantity%20A1))
  (bind _spawn_quantity_b1_3 (Variables|Spawn|GetSpawn%20Quantity%20B1))
  (bind _returnvalue (+ _spawn_quantity_a1 _spawn_quantity_b1))
  ;[1 1 1] Both players put their recipient at the middle spot
  (if (and (== (Variables|Game|GetRecipient%201) 1) (== (Variables|Game|GetRecipient%202) 1))
    (Variables|Game|SetP1RoundScore _spawn_quantity_b1_2)
    (Variables|Game|SetPlayer1Score (+ (Variables|Game|GetPlayer1Score) _spawn_quantity_b1_2))
    (Variables|Game|SetP2RoundScore _spawn_quantity_b1_3)
    (Variables|Game|SetPlayer2Score (+ (Variables|Game|GetPlayer2Score) _spawn_quantity_b1_3))
    (else
      ;[1 1 1] Only one player put the recipient at the middle spot
      (if (or (== (Variables|Game|GetRecipient%201) 1) (== (Variables|Game|GetRecipient%202) 1))
        (if (== (Variables|Game|GetRecipient%201) 1)
          (if (not (== (Variables|Game|GetRecipient%202) 2))
            (Variables|Game|SetPlayer2Score (+ (Variables|Game|GetPlayer2Score) _returnvalue))
            (Variables|Game|SetP2RoundScore _returnvalue))
          (elif (not (== (Variables|Game|GetRecipient%201) 2))
            (Variables|Game|SetPlayer1Score (+ _returnvalue (Variables|Game|GetPlayer1Score)))
            (Variables|Game|SetP1RoundScore _returnvalue)))
        (else
          ;[1 1 1] No one put the recipient at the middle spot
          (if (== (Variables|Game|GetRecipient%201) 2)
            (if (not (== (Variables|Game|GetRecipient%202) 2))
              (Variables|Game|SetP2RoundScore _spawn_quantity_a1_2)
              (Variables|Game|SetPlayer2Score (+ (Variables|Game|GetPlayer2Score) _spawn_quantity_a1_2)))
            (elif (== (Variables|Game|GetRecipient%202) 2)
              (Variables|Game|SetPlayer1Score (+ (Variables|Game|GetPlayer1Score) (Variables|Spawn|GetSpawn%20Quantity%20A1)))
              (Variables|Game|SetP1RoundScore (Variables|Spawn|GetSpawn%20Quantity%20A1))
              (else
                (Variables|Game|SetPlayer1Score (+ (Variables|Game|GetPlayer1Score) (Variables|Spawn|GetSpawn%20Quantity%20A1)))
                (Variables|Game|SetP1RoundScore (Variables|Spawn|GetSpawn%20Quantity%20A1))
                (Variables|Game|SetPlayer2Score (+ (Variables|Game|GetPlayer2Score) (Variables|Spawn|GetSpawn%20Quantity%20A1)))
                (Variables|Game|SetP2RoundScore (Variables|Spawn|GetSpawn%20Quantity%20A1))))))))))

(event Custom|Ask%20For%20Second%20Player%20Data
  ;[1 1 1] Game owner logic (server side on networking)
  ;;[1 0.07445 0] Ask The Second Play To Send Player Data
  (for _array_element (Variables|/Script/Engine.GameStateBase|GetPlayerArray (Game|GetGameState))
    (bind _aspstate (Utilities|Casting|CastToPState _array_element))
    (Default|AskforPlayerforData _aspstate)))

(event Custom|Update%20Round%20Score%20For%20Everyone
  ;[1 1 1] Game owner logic (server side on networking)
  ;;[3 0.03079 0] Tell all the players their scores updated
  (bind _asgame_instance_bal (Utilities|Casting|CastToGameInstance_BAL (Game|GetGameInstance)))
  (for _array_element (Variables|/Script/Engine.GameStateBase|GetPlayerArray (Game|GetGameState))
    (bind _aspstate (Utilities|Casting|CastToPState _array_element))
    (Default|UpdateRoundScore _aspstate (Variables|Game|GetP1RoundScore) (Variables|Game|GetP2RoundScore) (* (.number_of_rounds (Utilities|Struct|BreakMatchData (Variables|/Game/Blueprints/Common/GameInstance_BAL.GameInstance_BAL_C|GetMatchData _asgame_instance_bal))) (+ (.coop_points (Utilities|Struct|BreakMatchData (Variables|/Game/Blueprints/Common/GameInstance_BAL.GameInstance_BAL_C|GetMatchData _asgame_instance_bal))) (.no_coop_points (Utilities|Struct|BreakMatchData (Variables|/Game/Blueprints/Common/GameInstance_BAL.GameInstance_BAL_C|GetMatchData _asgame_instance_bal))))))))

(event Custom|Reset%20Fixed%20Begin%20Play
  ;[1 1 1] Game owner logic (server side on networking)
  ;;[1 1 1] Ask rotating plataforms to rotate according to players positions
  (Utilities|FlowControl|DoOnce false) ; enters at Reset
)

(event Custom|Show%20Score%20Widget
  ;[0.6245 0.2291 1] Scores
  (for _array_element (Variables|/Script/Engine.GameStateBase|GetPlayerArray (Game|GetGameState))
    (bind _aspstate (Utilities|Casting|CastToPState _array_element))
    (Default|ShowScoretoPlayer _aspstate)))

(event Custom|Clear%20Viewport
  ;[0.6245 0.2291 1] Scores
  (for _array_element (Variables|/Script/Engine.GameStateBase|GetPlayerArray (Game|GetGameState))
    (bind _aspstate (Utilities|Casting|CastToPState _array_element))
    (Default|ClearViewPortClients _aspstate)))

(event Custom|Play%20Again%20Event
  (params (IsServer :type Boolean) (Msg :type Integer))
  ;[1 0.01216 0] Send Play Again Msg  from one player to another
  (bind _result (Math|Integer|IncrementInt (Variables|Rematch|GetPlayerAgainMessages))
    (:%20%20
      (if (== _result 2)
        (Variables|Rematch|SetPlayerAgainMessages 0)
        (for _array_element (Variables|/Script/Engine.GameStateBase|GetPlayerArray (Game|GetGameState))
          (bind _aspstate (Utilities|Casting|CastToPState _array_element))
          (Default|ReceivePlayAgainMessagePState _aspstate Msg))
        (Utilities|FlowControl|Delay 0.2)
        (bind _asgame_instance_bal (Utilities|Casting|CastToGameInstance_BAL (Game|GetGameInstance)))
        (if (Variables|/Game/Blueprints/Common/GameInstance_BAL.GameInstance_BAL_C|GetResearchMode _asgame_instance_bal)
          (bind _returnvalue (UserInterface|CreateWidget "/Game/HUD/Menu/W_MatchData.W_MatchData_C"))
          (UserInterface|Viewport|AddtoViewport _returnvalue 0)
          (else
            (Utilities|FlowControl|Delay 3.0)
            (CallFunction|RematchEvent)))))))

(event Custom|Send%20Players%20Scores
  ;[0.1046 0.009134 0.004777] Send Players Scores
  (for _array_element (Variables|/Script/Engine.GameStateBase|GetPlayerArray (Game|GetGameState))
    (bind _aspstate (Utilities|Casting|CastToPState _array_element))
    (Default|SetPlayerScoresonClients _aspstate (|SetScoreData))))

(event Custom|New%20Round
  ;[1 1 1] Calculations after each round.
  (Utilities|FlowControl|Sequence
    (:then_0
      (CallFunction|SetRoundScore)
      (CallFunction|SetRoundInformation)
      (CallFunction|UpdateRoundScoreforEveryone)
      (CallFunction|RoundOverBroadcast))
    (:then_1
      (if (> (Variables|Game|GetRounds) 1)
        (Variables|Game|SetRounds (- (Variables|Game|GetRounds) 1))
        (Utilities|FlowControl|Delay 1.0)
        (CallFunction|ResetRound)
        (CallFunction|FixedBeginPlay)
        (else
          (CallFunction|EndGame))))))

(event Custom|Set%20Spawn%20Interval%20Time%20B
  (bind _spawn_quantity_b1 (Variables|Spawn|GetSpawn%20Quantity%20B1))
  (bind _preparation_time (Variables|Game|GetPreparation%20Time))
  (bind _returnvalue (Math|Conversions|ToFloat(Integer) _spawn_quantity_b1))
  (bind _returnvalue_2 (/ _preparation_time _returnvalue))
  ;[1 1 1] Game owner logic (server side on networking)
  ;;[1 1 1] Calculates the spawn interval time based on time and spawn quantity
  (if (> _returnvalue_2 (Variables|Game|GetSpawn%20Interval%20Treshold))
    (Variables|Game|SetSpawn%20Interval%20B (Variables|Game|GetSpawn%20Interval%20Treshold))
    (else
      (Variables|Game|SetSpawn%20Interval%20B _returnvalue_2))))

(event Custom|Reset%20Round
  ;[1 1 1] Game owner logic (server side on networking)
  ;;[1 0.9245 0] Resets The round variables
  (Variables|Game|SetRecipient%201 -1)
  (Variables|Game|SetRecipient%202 -1)
  (Variables|Game|SetP1RoundScore 0)
  (Variables|Game|SetP2RoundScore 0)
  (if (Variables|Rematch|GetRematch)
    (Variables|Rematch|SetRematch false)
    (Utilities|Array|Clear (Variables|Game|GetPlayers%20Data))
    (Utilities|Array|Clear (Variables|Game|GetRounds%20Data))
    (Variables|Game|SetPlayer1Score 0)
    (Variables|Game|SetPlayer2Score 0)
    (Utilities|FlowControl|Delay 1.0)
    (CallFunction|ClearViewport)
    (CallFunction|SetUpMatch)
    (CallFunction|RoundOverBroadcast)
    (CallFunction|ResetDoOnce)
    (Utilities|FlowControl|Delay 1.0)
    (CallFunction|FixedBeginPlay)
    (else
      (CallFunction|ResetDoOnce))))

(event Custom|Reset%20Do%20Once
  ;[1 1 1] Game owner logic (server side on networking)
  ;;[1 1 1] Ask rotating plataforms to rotate according to players positions
  (Utilities|FlowControl|DoOnce false) ; enters at Reset
)

(event Custom|Set%20Spawn%20interval%20Time%20A
  (bind _spawn_quantity_a1 (Variables|Spawn|GetSpawn%20Quantity%20A1))
  (bind _preparation_time (Variables|Game|GetPreparation%20Time))
  (bind _returnvalue (Math|Conversions|ToFloat(Integer) _spawn_quantity_a1))
  (bind _returnvalue_2 (/ _preparation_time _returnvalue))
  ;[1 1 1] Game owner logic (server side on networking)
  ;;[1 1 1] Calculates the spawn interval time based on time and spawn quantity
  (if (> _returnvalue_2 (Variables|Game|GetSpawn%20Interval%20Treshold))
    (Variables|Game|SetSpawn%20Interval%20A (Variables|Game|GetSpawn%20Interval%20Treshold))
    (else
      (Variables|Game|SetSpawn%20Interval%20A _returnvalue_2))))

(event Custom|On%20Preparation
  ;[1 1 1] Game owner logic (server side on networking)
  ;;[1 1 1] On Preparation Event that calls all clients to set their variables
  (for _array_element (Variables|/Script/Engine.GameStateBase|GetPlayerArray (Game|GetGameState))
    (bind _aspstate (Utilities|Casting|CastToPState _array_element))
    (CallFunction|PreparationTimeBegin)
    (CallFunction|SetSpawnIntervalTimeA)
    (CallFunction|SetSpawnIntervalTimeB)
    (Default|PreparationMatch _aspstate (Variables|Spawn|GetSpawn%20Index%201) (Variables|Spawn|GetSpawn%20Index%202) (Variables|Spawn|GetSpawn%20Index%203) (Variables|Spawn|GetSpawn%20Index%204) (Variables|Spawn|GetNeutral%20Position) (Variables|Game|GetSpawn%20Interval%20A) (Variables|Game|GetSpawn%20Interval%20B) (Variables|Spawn|GetSpawn%20Quantity%20A1) (Variables|Spawn|GetSpawn%20Quantity%20B1) (Variables|Game|GetPreparation%20Time))))

(event Custom|Rematch%20Event
  ;[1 0.01216 0] Send Play Again Msg  from one player to another
  (Variables|Rematch|SetRematch true)
  (CallFunction|ResetRound))

(event Custom|Set%20up%20match
  ;[1 1 1] Set up the information right in the begining of the match
  (bind _asgame_instance_bal (Utilities|Casting|CastToGameInstance_BAL (Game|GetGameInstance)))
  (Utilities|Array|Add (Variables|Game|GetPlayers%20Data) (Variables|/Game/Blueprints/Common/GameInstance_BAL.GameInstance_BAL_C|GetPlayerData _asgame_instance_bal))
  (Variables|Spawn|SetSpawn%20Quantity%20B1 (.coop_points (Utilities|Struct|BreakMatchData (Variables|/Game/Blueprints/Common/GameInstance_BAL.GameInstance_BAL_C|GetMatchData _asgame_instance_bal))))
  (Variables|Spawn|SetSpawn%20Quantity%20A1 (.no_coop_points (Utilities|Struct|BreakMatchData (Variables|/Game/Blueprints/Common/GameInstance_BAL.GameInstance_BAL_C|GetMatchData _asgame_instance_bal))))
  (Variables|Game|SetStrategy (.strategy (Utilities|Struct|BreakMatchData (Variables|/Game/Blueprints/Common/GameInstance_BAL.GameInstance_BAL_C|GetMatchData _asgame_instance_bal))))
  (Variables|Game|SetRounds (.number_of_rounds (Utilities|Struct|BreakMatchData (Variables|/Game/Blueprints/Common/GameInstance_BAL.GameInstance_BAL_C|GetMatchData _asgame_instance_bal)))))

(event Custom|Preparation%20Time%20End
  ;[1 1 1] Game owner logic (server side on networking)
  ;;[1 1 1] Binding timer for preparation phase where players will have a time to choose a spot for their recipient
  (Variables|Game|SetRoundState "NewEnumerator1")
  (Utilities|Time|ClearandInvalidateTimerbyHandle (stale Custom|Preparation%20Time%20Begin _returnvalue))
  (CallFunction|OnPreparationEndBroadCast))

(event Custom|End%20Game
  ;[1 1 1] End Game
  (bind _asgame_instance_bal (Utilities|Casting|CastToGameInstance_BAL (Game|GetGameInstance)))
  (Variables|Game|SetMatch%20Data (|MakeMatchData_2 (Variables|/Game/Blueprints/Common/GameInstance_BAL.GameInstance_BAL_C|GetMatchData _asgame_instance_bal)))
  (CallFunction|SendPlayersScores)
  (CallFunction|ShowScoreWidget)
  (if (Variables|/Game/Blueprints/Common/GameInstance_BAL.GameInstance_BAL_C|GetResearchMode _asgame_instance_bal)
    (CallFunction|AskforSecondPlayerData)
    (Utilities|FlowControl|Delay 1.0)
    (bind _returnvalue (Class|SaveandLoadFiles|SaveJsontoFile (Variables|Game|GetMatch%20Data)))
    (if _returnvalue
      (Development|PrintString "Salvou")
      (else
        (Development|PrintString "não salvou")))
    (else
      (Development|PrintString "no research mode"))))

(event Custom|Set%20Second%20Player%20Information
  (params (Second%20Player%20Data :type Player%20Data%20Structure))
  (bind _players_data (Variables|Game|GetPlayers%20Data))
  ;[1 1 1] Set Second Player Information
  (Utilities|Array|Add _players_data Second%20Player%20Data)
  (Variables|Game|SetMatch%20Data (|SetPlayerDataForPlayer2info (Variables|Game|GetMatch%20Data) _players_data)))

(event Custom|Receive%20client%20update
  (params (NewRecipientLocation :type Integer) (isServer :type Boolean))
  (bind _returnvalue (Game|GetGameState))
  (bind _playerarray (Variables|/Script/Engine.GameStateBase|GetPlayerArray _returnvalue))
  (bind _item (Utilities|Array|Get(acopy) _playerarray))
  (bind _item_2 (Utilities|Array|Get(acopy) _playerarray 1))
  ;[1 1 1] Game owner logic (server side on networking)
  ;;[1 1 1] Recieving players recipients updated pose after preparation ends
  (if isServer
    (bind _output_get (Variables|Game|SetRecipient%201 NewRecipientLocation))
    (bind _asbalanca_player_controller (Utilities|Casting|CastToBalanca_PlayerController (Components|GetOwner _item_2)))
    (if (not (Pawn|IsLocalController _asbalanca_player_controller))
      (bind _aspstate (Utilities|Casting|CastToPState _item_2))
      (Default|UpdatePlayer2Recipient _aspstate _output_get)
      (else
        (bind _aspstate_2 (Utilities|Casting|CastToPState (Utilities|Array|Get(acopy) _playerarray)))
        (Default|UpdatePlayer2Recipient _aspstate_2 _output_get)))
    (else
      (bind _output_get_2 (Variables|Game|SetRecipient%202 NewRecipientLocation))
      (bind _asbalanca_player_controller_2 (Utilities|Casting|CastToBalanca_PlayerController (Components|GetOwner _item)))
      (if (Pawn|IsLocalController _asbalanca_player_controller_2)
        (bind _aspstate_3 (Utilities|Casting|CastToPState _item))
        (Default|UpdatePlayer2Recipient _aspstate_3 _output_get_2)
        (else
          (bind _aspstate_4 (Utilities|Casting|CastToPState (Utilities|Array|Get(acopy) _playerarray 1)))
          (Default|UpdatePlayer2Recipient _aspstate_4 _output_get_2))))))

(event Custom|Preparation%20Time%20Begin
  ;[1 1 1] Game owner logic (server side on networking)
  ;;[1 1 1] Binding timer for preparation phase where players will have a time to choose a spot for their recipient
  (bind _returnvalue (Utilities|Time|SetTimerbyEvent (delegate Custom|Preparation%20Time%20End) (Variables|Game|GetPreparation%20Time))))

(event Custom|Set%20Round%20Information
  ;[1 1 1] Sets Round Data every end of round
  (bind _asgame_instance_bal (Utilities|Casting|CastToGameInstance_BAL (Game|GetGameInstance)))
  (Utilities|Array|Add (Variables|Game|GetRounds%20Data) (|SetRoundData (|GetMaxNumberOfRounds (Variables|/Game/Blueprints/Common/GameInstance_BAL.GameInstance_BAL_C|GetMatchData _asgame_instance_bal)))))

(event Custom|Fixed%20Begin%20Play
  ;[1 1 1] Game owner logic (server side on networking)
  ;;[1 1 1] Event that check if all players are connected to start the round and ask them to set their required references
  (Utilities|FlowControl|Sequence
    (:then_0
      (Utilities|FlowControl|DoOnce false
        (:Completed
          (CallFunction|SetUpMatch))))
    (:then_1
      (Variables|Game|SetRoundState "NewEnumerator0")
      (CallFunction|OnPreparation)
      (for _array_element (Variables|/Script/Engine.GameStateBase|GetPlayerArray (Game|GetGameState))
        (bind _aspstate (Utilities|Casting|CastToPState _array_element))
        (Default|GetRotatingPlataform _aspstate)))))

(event EventOnLogout
  (params (ExitingController :type Controller%20Object%20Reference))
  (if (not (Pawn|IsLocalController ExitingController))
    (bind _returnvalue (UserInterface|CreateWidget "/Game/HUD/Menu/W_MenuMessages.W_MenuMessages_C"))
    (UserInterface|Viewport|AddtoViewport _returnvalue 0)
    (Rendering|Components|TextRender|SetText (Variables|/Game/HUD/Menu/W_MenuMessages.W_MenuMessages_C|GetTxt_MenuMessages _returnvalue) "Player 2 saiu")))

(event EventBeginPlay
  (bind _returnvalue (Game|SpawnActorfromClass "/Game/Blueprints/Common/BlueprintHttpActor.BlueprintHttpActor_C" (Math|Transform|MakeTransform "0, 0, 0") "Undefined" 0 0))
  (Variables|HTTP|SetHttpActor _returnvalue))

(event EventTick
  (params (DeltaSeconds :type Float%20%28single-precision%29))
  ;[1 1 1] Game owner logic (server side on networking)
  ;;[1 1 1] Ask rotating plataforms to rotate according to players positions
  (Utilities|FlowControl|Sequence
    (:then_0
      (if (and (!= (Variables|Game|GetRecipient%201) -1) (!= (Variables|Game|GetRecipient%202) -1))
        (Utilities|FlowControl|DoOnce false
          (:Completed
            (CallFunction|RotatePlayersPlatform)
            (Utilities|FlowControl|Delay 5.0)
            (CallFunction|NewRound)))))
    (:then_1
      (if (== (Utilities|Array|Length (Variables|/Script/Engine.GameStateBase|GetPlayerArray (Game|GetGameState))) 2)
        (Utilities|FlowControl|DoOnce false
          (:Completed
            (CallFunction|FixedBeginPlay)))))))

(fn ConstructionScript)

(fn RotatePlayersPlatform
  (for _array_element (Variables|/Script/Engine.GameStateBase|GetPlayerArray (Game|GetGameState))
    (bind _aspstate (Utilities|Casting|CastToPState _array_element))
    (Default|RotatePlataformwithPositions _aspstate (Variables|Game|GetRecipient%201) (Variables|Game|GetRecipient%202)))
  (return))

(fn RoundOverBroadcast
  (for _array_element (Variables|/Script/Engine.GameStateBase|GetPlayerArray (Game|GetGameState))
    (bind _aspstate (Utilities|Casting|CastToPState _array_element))
    (Default|RoundOver _aspstate))
  (return))