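; Menu game mode that drives the front-end flow from main menu through player info and match data screens into single-player Balanca_Map.
; BeginPlay spawns the HTTP actor, shows the main menu, clears game instance info and loads JSON options into it.
; Custom events swap screens by toggling widget visibility, and starting a game opens the map after a delay.
; A helper builds match-data URL options, but the level opens with empty options.
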(event Custom|Play
  (bind _menuhud (Variables|Default|GetMenuHud))
  ;[1 1 1] Change the menu to player's info menu
  (if (Widget|IsVisible _menuhud)
    (Widget|SetVisibility _menuhud "Hidden"))
  (bind _returnvalue (UserInterface|CreateWidget "/Game/HUD/Menu/W_PlayerInfo.W_PlayerInfo_C"))
  (Variables|Default|SetPlayerInfoHud _returnvalue)
  (UserInterface|Viewport|AddtoViewport _returnvalue 0))

(event Custom|Back%20To%20Main%20Menu
  (bind _playerinfohud (Variables|Default|GetPlayerInfoHud))
  (bind _menuhud (Variables|Default|GetMenuHud))
  (bind _matchdatainput (Variables|Default|GetMatchDataInput))
  ;[1 1 1] Clear all the widgets and go back to main menu
  (Utilities|IsValid _playerinfohud
    (:Is%20Valid
      (Widget|SetVisibility _playerinfohud "Hidden"))
    (:Is%20Not%20Valid
      _))
  (Utilities|IsValid _matchdatainput
    (:Is%20Valid
      (Widget|SetVisibility _matchdatainput "Hidden"))
    (:Is%20Not%20Valid
      (Utilities|IsValid _menuhud
        (:Is%20Valid
          _))))
  (Widget|SetVisibility _menuhud "Visible"))

(event Custom|CustomEvent)

(event Custom|Match%20Data%20Input
  ;[1 1 1] Show the menu to put match data information
  (Widget|SetVisibility (Variables|Default|GetPlayerInfoHud) "Hidden")
  (Utilities|IsValid (Variables|Default|GetMatchDataInput)
    (:Is%20Valid
      (Widget|SetVisibility (Variables|Default|GetMatchDataInput) "Visible"))
    (:Is%20Not%20Valid
      (bind _returnvalue (UserInterface|CreateWidget "/Game/HUD/Menu/W_MatchData.W_MatchData_C"))
      (Variables|Default|SetMatchDataInput _returnvalue)
      (UserInterface|Viewport|AddtoViewport _returnvalue 0))))

(event Custom|Start%20Single%20Player%20Game
  ;[1 1 1] Start the single player game
  (Widget|SetVisibility (Variables|Default|GetMatchDataInput) "Hidden")
  (Utilities|FlowControl|Delay 2.0)
  (Game|OpenLevel(byName) "Balanca_Map"))

(event EventBeginPlay
  ;[1 1 1] Creates the menu widget
  (Game|SpawnActorfromClass "/Game/Blueprints/Common/BlueprintHttpActor.BlueprintHttpActor_C" (|Transform) "Undefined" 0 0)
  (bind _returnvalue (UserInterface|CreateWidget "/Game/HUD/Menu/W_Menu.W_Menu_C"))
  (Variables|Default|SetMenuHud _returnvalue)
  (UserInterface|Viewport|AddtoViewport _returnvalue 0)
  (bind _asgame_instance_bal (Utilities|Casting|CastToGameInstance_BAL (Game|GetGameInstance)))
  (Default|ClearInfo _asgame_instance_bal)
  (bind _returnvalue_2 (Class|SaveandLoadFiles|LoadOptionsJsontoStruct))
  (Variables|/Game/Blueprints/Common/GameInstance_BAL.GameInstance_BAL_C|SetOptionsData _asgame_instance_bal _returnvalue_2))

(event EventTick
  (params (DeltaSeconds :type Float%20%28single-precision%29)))

(fn ConstructionScript)

(fn GetStringOptionsforSinglePlayer
  (bind _asgame_instance_bal (Utilities|Casting|CastToGameInstance_BAL (Game|GetGameInstance))
    (:then
      (Development|PrintString (Utilities|String|Append "?Rounds=" (Utilities|String|ToString(Integer) (.number_of_rounds (Utilities|Struct|BreakMatchData (Variables|/Game/Blueprints/Common/GameInstance_BAL.GameInstance_BAL_C|GetMatchData _asgame_instance_bal)))) "?QuantityB=" (Utilities|String|ToString(Integer) (.coop_points (Utilities|Struct|BreakMatchData (Variables|/Game/Blueprints/Common/GameInstance_BAL.GameInstance_BAL_C|GetMatchData _asgame_instance_bal)))) "?QuantityA=" (Utilities|String|ToString(Integer) (.no_coop_points (Utilities|Struct|BreakMatchData (Variables|/Game/Blueprints/Common/GameInstance_BAL.GameInstance_BAL_C|GetMatchData _asgame_instance_bal)))) "?Strategy=" (Utilities|String|ToString(Integer) (.strategy (Utilities|Struct|BreakMatchData (Variables|/Game/Blueprints/Common/GameInstance_BAL.GameInstance_BAL_C|GetMatchData _asgame_instance_bal))))))
      (return (Utilities|String|Append "?Rounds=" (Utilities|String|ToString(Integer) (.number_of_rounds (Utilities|Struct|BreakMatchData (Variables|/Game/Blueprints/Common/GameInstance_BAL.GameInstance_BAL_C|GetMatchData _asgame_instance_bal)))) "?QuantityB=" (Utilities|String|ToString(Integer) (.coop_points (Utilities|Struct|BreakMatchData (Variables|/Game/Blueprints/Common/GameInstance_BAL.GameInstance_BAL_C|GetMatchData _asgame_instance_bal)))) "?QuantityA=" (Utilities|String|ToString(Integer) (.no_coop_points (Utilities|Struct|BreakMatchData (Variables|/Game/Blueprints/Common/GameInstance_BAL.GameInstance_BAL_C|GetMatchData _asgame_instance_bal)))) "?Strategy=" (Utilities|String|ToString(Integer) (.strategy (Utilities|Struct|BreakMatchData (Variables|/Game/Blueprints/Common/GameInstance_BAL.GameInstance_BAL_C|GetMatchData _asgame_instance_bal)))))))
    (:CastFailed
      (return "?Rounds=2"))))