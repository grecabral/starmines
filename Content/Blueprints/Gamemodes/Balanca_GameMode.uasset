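; Game mode for Balança, a round-based cooperate-or-not game in which the player faces a strategy-driven bot.
; A timed preparation phase drops point objects, then the bot's recipient spawns from a fixed, history-based or random strategy and the platform rotates.
; Payoff rules score both choices into GameInstance_BAL, which carries history across the level reload that starts each round.
; The last round saves match data as JSON and shows the score widget.
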(event Custom|On%20Preparation%20Over
  ;[1 1 1] Preparation end and broadcast it to all clients
  (bind _outactors (Actor|GetAllActorsOfClass "/Game/Blueprints/Common/Balanca_RotatingPlataform.Balanca_RotatingPlataform_C"))
  (bind _output_get (Variables|Actors|SetRotatePlatform (Utilities|Array|Get(acopy) _outactors)))
  (CallFunction|SpawnSecondRecipient)
  (Default|EvaluateRotation _output_get (Variables|Game|GetRecipient%201) (Variables|Game|GetRecipient%202))
  (Utilities|FlowControl|Delay 5.0)
  (CallFunction|NewRound))

(event Custom|Spawn%20Recipient
  (params (Location :type Vector))
  ;[1 1 1] Spanws The player's recipient
  (Game|SpawnActorfromClass "/Game/Blueprints/SinglePlayer/Balanca_RecipientSP.Balanca_RecipientSP_C" (Math|Transform|MakeTransform (Variables|Spawn|GetNeutral%20Point) "0,90.000000, 0" "-1.000000,1.000000,1") "Undefined" 0 true 0)
  (Game|SpawnActorfromClass "/Game/Blueprints/Common/Curtain.Curtain_C" (Math|Transform|MakeTransform (Variables|Spawn|Getlocation%20curtain) "0,0.000000, 0") "AlwaysSpawn" 0 0)
  (Variables|Game|SetPlayerPosition "NewEnumerator2")
  (Variables|Game|SetRecipient%201 2))

(event Custom|Get%20All%20Info%20Widgets
  ;[1 1 1] Get All widgets at viewport
  (bind _foundwidgets (Widget|GetAllWidgetsOfClass "/Game/HUD/Menu/W_PlayerInfo.W_PlayerInfo_C" true))
  (for _array_element _foundwidgets
    _)
  (bind _foundwidgets_2 (Widget|GetAllWidgetsOfClass "/Game/HUD/Menu/W_MatchData.W_MatchData_C" true))
  (for _array_element_2 _foundwidgets_2
    _))

(event Custom|Spawn%20A%20Objects
  ;[1 1 1] Spawns the falling objects
  (if (== (Variables|Spawn|GetSpawn%20Quantity%20A1) (Variables|Spawn|GetNumber%20A%20Spawned))
    (Utilities|Time|ClearandInvalidateTimerbyHandle (stale Custom|Spawn%20Falling%20Objects _returnvalue))
    (else
      (Math|Integer|IncrementInt (Variables|Spawn|GetNumber%20A%20Spawned)
        (:%20%20
          (Game|SpawnActorfromClass "/Game/Blueprints/SinglePlayer/Balanca_FallingObject_SP.Balanca_FallingObject_SP_C" (Math|Conversions|ToTransform(Vector) (Transformation|GetActorLocation (Utilities|Array|Get(acopy) (Variables|Game|GetSpawn%20Points) (Variables|Spawn|GetSpawn%20Index%201)))) "Undefined" (Game|Player|GetPlayerPawn 0) 0)
          (Game|SpawnActorfromClass "/Game/Blueprints/SinglePlayer/Balanca_FallingObject_SP.Balanca_FallingObject_SP_C" (Math|Conversions|ToTransform(Vector) (Variables|Spawn|GetA2%20Location)) "Undefined" 0 0))))))

(event Custom|Spawn%20B%20Objects
  ;[1 1 1] Spawns the falling objects
  (if (== (Variables|Spawn|GetSpawn%20Quantity%20B1) (Variables|Spawn|GetNumber%20B%20Spawned))
    (Utilities|Time|ClearandInvalidateTimerbyHandle (stale Custom|Spawn%20Falling%20Objects _returnvalue_2))
    (else
      (Math|Integer|IncrementInt (Variables|Spawn|GetNumber%20B%20Spawned)
        (:%20%20
          (Game|SpawnActorfromClass "/Game/Blueprints/SinglePlayer/Balanca_FallingObject_SP.Balanca_FallingObject_SP_C" (Math|Conversions|ToTransform(Vector) (Transformation|GetActorLocation (Utilities|Array|Get(acopy) (Variables|Game|GetSpawn%20Points) (Variables|Spawn|GetSpawn%20Index%202)))) "Undefined" 0 0)
          (Game|SpawnActorfromClass "/Game/Blueprints/SinglePlayer/Balanca_FallingObject_SP.Balanca_FallingObject_SP_C" (Math|Conversions|ToTransform(Vector) (Variables|Spawn|GetB2%20Location)) "Undefined" 0 0))))))

(event Custom|New%20Round
  ;[1 1 1] New Round Preparation
  (bind _asgame_instance_bal (Utilities|Casting|CastToGameInstance_BAL (Game|GetGameInstance)))
  (CallFunction|SetPlayerRoundScore)
  (bind _rounddata (CallFunction|SetRoundData _asgame_instance_bal))
  (Utilities|Array|Add (Variables|/Game/Blueprints/Common/GameInstance_BAL.GameInstance_BAL_C|GetRoundData _asgame_instance_bal) _rounddata)
  (CallFunction|AddScoretoScoreHolder)
  (CallFunction|SetTotalScore)
  (if (> (Variables|Game|GetRounds) 1)
    (bind _result (Math|Integer|DecrementInt (Variables|Game|GetRounds))
      (:%20%20
        (Variables|/Game/Blueprints/Common/GameInstance_BAL.GameInstance_BAL_C|SetRounds _asgame_instance_bal _result)
        (bind _returnvalue (Game|GetCurrentLevelName true))
        ;;[1 1 1] Computando score
        (Utilities|FlowControl|Delay 3.0)
        (Game|OpenLevel(byName) (Utilities|String|StringToName _returnvalue))))
    (else
      (CallFunction|EndGame))))

(event Custom|Set%20Spawn%20Interval%20Time%20B
  (bind _spawn_quantity_b1 (Variables|Spawn|GetSpawn%20Quantity%20B1))
  (bind _preparation_time (Variables|Game|GetPreparation%20Time))
  (bind _returnvalue (Math|Conversions|ToFloat(Integer) _spawn_quantity_b1))
  (bind _returnvalue_2 (/ _preparation_time _returnvalue))
  ;[1 1 1] Calculates the spawn interval time based on time and spawn quantity
  (if (> _returnvalue_2 (Variables|Game|GetSpawn%20Interval%20Treshold))
    (Variables|Game|SetSpawn%20Interval%20B (Variables|Game|GetSpawn%20Interval%20Treshold))
    (else
      (Variables|Game|SetSpawn%20Interval%20B _returnvalue_2))))

(event Custom|Set%20Spawn%20interval%20Time%20A
  (bind _spawn_quantity_a1 (Variables|Spawn|GetSpawn%20Quantity%20A1))
  (bind _preparation_time (Variables|Game|GetPreparation%20Time))
  (bind _returnvalue (Math|Conversions|ToFloat(Integer) _spawn_quantity_a1))
  (bind _returnvalue_2 (/ _preparation_time _returnvalue))
  ;[1 1 1] Calculates the spawn interval time based on time and spawn quantity
  (if (> _returnvalue_2 (Variables|Game|GetSpawn%20Interval%20Treshold))
    (Variables|Game|SetSpawn%20Interval%20A (Variables|Game|GetSpawn%20Interval%20Treshold))
    (else
      (Variables|Game|SetSpawn%20Interval%20A _returnvalue_2))))

(event Custom|Spawn%20Falling%20Objects
  (params (Quantity%20A1 :type Integer) (Quantity%20B1 :type Integer))
  ;[1 1 1] Spawns the falling objects
  (bind _output_get (Variables|Spawn|SetSpawn%20Quantity%20A1 Quantity%20A1))
  (Variables|Spawn|SetSpawn%20Quantity%20A2 _output_get)
  (bind _output_get_2 (Variables|Spawn|SetSpawn%20Quantity%20B1 Quantity%20B1))
  (Variables|Spawn|SetSpawn%20Quantity%20B2 _output_get_2)
  (CallFunction|SpawnAObjects)
  (CallFunction|SpawnBObjects)
  (bind _returnvalue (Utilities|Time|SetTimerbyEvent (delegate Custom|Spawn%20A%20Objects) (Variables|Game|GetSpawn%20Interval%20A) true))
  (bind _returnvalue_2 (Utilities|Time|SetTimerbyEvent (delegate Custom|Spawn%20B%20Objects) (Variables|Game|GetSpawn%20Interval%20B) true)))

(event Custom|On%20Pre-preparation%20Start
  ;[1 1 1] Preaparation for the start preparation
  (Utilities|FlowControl|Sequence
    (:then_0
      (Variables|Game|SetRoundState "NewEnumerator0")
      (Variables|Spawn|SetSpawn%20Index%201 0)
      (Variables|Spawn|SetSpawn%20Index%202 1)
      (Variables|Spawn|SetSpawn%20Index%203 2)
      (Variables|Spawn|SetSpawn%20Index%204 3)
      (bind _outactors (Actor|GetAllActorswithTag "SpawnTargetPoint"))
      (for _array_element _outactors
        (bind _astarget_point (Utilities|Casting|CastToTargetPoint _array_element))
        (switch string (Utilities|GetDisplayName _astarget_point)
          (:TargetPoint1
            (Utilities|Array|SetArrayElem (Variables|Game|GetSpawn%20Points) (Variables|Spawn|GetSpawn%20Index%201) _astarget_point))
          (:TargetPoint2
            (Utilities|Array|SetArrayElem (Variables|Game|GetSpawn%20Points) (Variables|Spawn|GetSpawn%20Index%202) _astarget_point))
          (:TargetPoint3
            (Utilities|Array|SetArrayElem (Variables|Game|GetSpawn%20Points) (Variables|Spawn|GetSpawn%20Index%203) _astarget_point))
          (:TargetPoint4
            (Utilities|Array|SetArrayElem (Variables|Game|GetSpawn%20Points) (Variables|Spawn|GetSpawn%20Index%204) _astarget_point)))))
    (:then_1
      (CallFunction|SetSpawnIntervalTimeA)
      (CallFunction|SetSpawnIntervalTimeB)
      (CallFunction|SpawnRecipient (Variables|Spawn|Getlocation%20curtain)))
    (:then_2
      ;;[1 1 1] !
      (bind _returnvalue (UserInterface|CreateWidget "/Game/HUD/W_GameStartWarning.W_GameStartWarning_C"))
      (UserInterface|Viewport|AddtoViewport _returnvalue 5)
      (Utilities|FlowControl|Delay 1.5)
      (Widget|RemovefromParent _returnvalue))))

(event Custom|Spawn%20Second%20Recipient
  ;[1 1 1] Bot's recipient spawn accordingly with chosen strategy
  (bind _asgame_instance_bal (Utilities|Casting|CastToGameInstance_BAL (Game|GetGameInstance)))
  (switch Utilities|FlowControl|Switch|SwitchonEnum_Strategies (Utilities|Enum|ByteToEnumEnum_Strategies (Math|Conversions|ToByte(Integer) (Variables|Game|GetBotStrategy)))
    (:NewEnumerator0
      (Variables|Game|SetRecipient%202 1))
    (:NewEnumerator1
      (Variables|Game|SetRecipient%202 0))
    (:NewEnumerator2
      (if (== (Variables|Game|GetRounds) (Variables|/Game/Blueprints/Common/GameInstance_BAL.GameInstance_BAL_C|GetMax%20Rounds _asgame_instance_bal))
        (Variables|Game|SetRecipient%202 1)
        (elif (== (|Getplayerpositiononlastround (Utilities|Array|Get(acopy) (Variables|/Game/Blueprints/Common/GameInstance_BAL.GameInstance_BAL_C|GetRoundData _asgame_instance_bal) (- (- (Variables|/Game/Blueprints/Common/GameInstance_BAL.GameInstance_BAL_C|GetMax%20Rounds _asgame_instance_bal) (Variables|Game|GetRounds)) 1))) 2)
          (Variables|Game|SetRecipient%202 (|GetSecondPlayerlastposition (Utilities|Array|Get(acopy) (Variables|/Game/Blueprints/Common/GameInstance_BAL.GameInstance_BAL_C|GetRoundData _asgame_instance_bal) (- (- (Variables|/Game/Blueprints/Common/GameInstance_BAL.GameInstance_BAL_C|GetMax%20Rounds _asgame_instance_bal) (Variables|Game|GetRounds)) 1))))
          (else
            (Variables|Game|SetRecipient%202 (|Getplayerpositiononlastround (Utilities|Array|Get(acopy) (Variables|/Game/Blueprints/Common/GameInstance_BAL.GameInstance_BAL_C|GetRoundData _asgame_instance_bal) (- (- (Variables|/Game/Blueprints/Common/GameInstance_BAL.GameInstance_BAL_C|GetMax%20Rounds _asgame_instance_bal) (Variables|Game|GetRounds)) 1))))))))
    (:NewEnumerator3
      (if (not (> (Variables|/Game/Blueprints/Common/GameInstance_BAL.GameInstance_BAL_C|GetMax%20Rounds _asgame_instance_bal) 2))
        (Variables|Game|SetRecipient%202 1)
        (elif (not (> (- (Variables|/Game/Blueprints/Common/GameInstance_BAL.GameInstance_BAL_C|GetMax%20Rounds _asgame_instance_bal) (Variables|Game|GetRounds)) 1))
          (Variables|Game|SetRecipient%202 1)
          (elif (and (== (|Getplayerpositiononlastround (Utilities|Array|Get(acopy) (Variables|/Game/Blueprints/Common/GameInstance_BAL.GameInstance_BAL_C|GetRoundData _asgame_instance_bal) (- (- (Variables|/Game/Blueprints/Common/GameInstance_BAL.GameInstance_BAL_C|GetMax%20Rounds _asgame_instance_bal) (Variables|Game|GetRounds)) 1))) 0) (== (|Getplayerpositiononlastround_2 (Utilities|Array|Get(acopy) (Variables|/Game/Blueprints/Common/GameInstance_BAL.GameInstance_BAL_C|GetRoundData _asgame_instance_bal) (- (- (Variables|/Game/Blueprints/Common/GameInstance_BAL.GameInstance_BAL_C|GetMax%20Rounds _asgame_instance_bal) (Variables|Game|GetRounds)) 2))) 0))
            (Variables|Game|SetRecipient%202 0)
            (else
              (Variables|Game|SetRecipient%202 1))))))
    (:NewEnumerator4
      (Variables|Game|SetRecipient%202 (Math|Random|RandomIntegerinRange 0 1))))
  (bind _returnvalue (Game|SpawnActorfromClass "/Game/Blueprints/SinglePlayer/Balanca_RecipientSP.Balanca_RecipientSP_C" (Utilities|Select :Index (Variables|Game|GetRecipient%202) :Option%200 (Math|Transform|MakeTransform (Variables|Snapping|GetSnapping%20Non%20Coop%20Position) "0,90.000000, 0" "1,1.000000,1.000000") :Option%201 (Math|Transform|MakeTransform (Variables|Snapping|GetSnapping%20Coop%20Position) "0,90.000000, 0" "1,1.000000,1.000000")) "Undefined" 0 false 0))
  (if (== (Variables|Game|GetRecipient%202) 1)
    (Transformation|AttachActorToActor _returnvalue (Variables|Actors|GetRotatePlatform) "None" "KeepWorld" "KeepWorld" "KeepWorld" true)))

(event Custom|Back%20To%20Main%20Menu
  ;[1 1 1] Event to return to main menu
  (Widget|RemovefromParent (Variables|Game|GetShowScoreWidget))
  (Game|OpenLevel(byName) "Menu"))

(event Custom|Set%20Player%20Round%20Score
  (bind _spawn_quantity_a1 (Variables|Spawn|GetSpawn%20Quantity%20A1))
  (bind _spawn_quantity_b1 (Variables|Spawn|GetSpawn%20Quantity%20B1))
  (bind _spawn_quantity_b1_2 (Variables|Spawn|GetSpawn%20Quantity%20B1))
  (bind _spawn_quantity_a1_2 (Variables|Spawn|GetSpawn%20Quantity%20A1))
  (bind _returnvalue (+ _spawn_quantity_a1 _spawn_quantity_b1))
  ;[1 1 1] Both players put their recipient at the co-op spot
  (if (and (== (Variables|Game|GetRecipient%201) 1) (== (Variables|Game|GetRecipient%202) 1))
    (CallFunction|SetScoresbyRound _spawn_quantity_b1_2 _spawn_quantity_b1_2)
    (else
      ;[1 1 1] Only one player put the recipient at the co-op spot
      (if (or (== (Variables|Game|GetRecipient%201) 1) (== (Variables|Game|GetRecipient%202) 1))
        (if (== (Variables|Game|GetRecipient%201) 1)
          (CallFunction|SetScoresbyRound 0 _returnvalue)
          (elif (not (== (Variables|Game|GetRecipient%201) 2))
            (CallFunction|SetScoresbyRound _returnvalue)))
        (else
          ;[1 1 1] Comment
          ;;[1 1 1] Player 1 let the recipient at neutral spot and Player 2 put the recipient at non co-op spot
          (if (== (Variables|Game|GetRecipient%201) 2)
            (CallFunction|SetScoresbyRound 0 (Variables|Spawn|GetSpawn%20Quantity%20A1))
            (else
              ;[1 1 1] Both Players put the recipient at non co-op spot
              (CallFunction|SetScoresbyRound _spawn_quantity_a1_2 _spawn_quantity_a1_2))))))))

(event Custom|Preparation%20Time%20End
  ;[1 1 1] Binding timer for preparation phase where players will have a time to choose a spot for their recipient
  (Variables|Game|SetRoundState "NewEnumerator1")
  (Utilities|Time|ClearandInvalidateTimerbyHandle (stale Custom|Preparation%20Time%20Begin _returnvalue))
  (Default|CallPreparationOverDispatcher)
  (CallFunction|OnPreparationOver))

(event Custom|End%20Game
  ;[1 1 1] Eng Match responsible for get all the match information and send it to the server
  ;;[0 0.1739 1] Make the match Data
  (bind _asgame_instance_bal (Utilities|Casting|CastToGameInstance_BAL (Game|GetGameInstance)))
  (bind _output_get (Variables|/Game/Blueprints/Common/GameInstance_BAL.GameInstance_BAL_C|SetMatchData _asgame_instance_bal (|Setmatchdatastruct (Utilities|Array|MakeArray (Variables|/Game/Blueprints/Common/GameInstance_BAL.GameInstance_BAL_C|GetPlayerData _asgame_instance_bal)) (.number_of_rounds (|GetMatchDatainfofromgameinstance (Variables|/Game/Blueprints/Common/GameInstance_BAL.GameInstance_BAL_C|GetMatchData _asgame_instance_bal))) (.coop_points (|GetMatchDatainfofromgameinstance (Variables|/Game/Blueprints/Common/GameInstance_BAL.GameInstance_BAL_C|GetMatchData _asgame_instance_bal))) (.no_coop_points (|GetMatchDatainfofromgameinstance (Variables|/Game/Blueprints/Common/GameInstance_BAL.GameInstance_BAL_C|GetMatchData _asgame_instance_bal))) (.difficulty (|GetMatchDatainfofromgameinstance (Variables|/Game/Blueprints/Common/GameInstance_BAL.GameInstance_BAL_C|GetMatchData _asgame_instance_bal))) (.strategy (|GetMatchDatainfofromgameinstance (Variables|/Game/Blueprints/Common/GameInstance_BAL.GameInstance_BAL_C|GetMatchData _asgame_instance_bal))) (Variables|/Game/Blueprints/Common/GameInstance_BAL.GameInstance_BAL_C|GetRoundData _asgame_instance_bal) (.gameFlag (|GetMatchDatainfofromgameinstance (Variables|/Game/Blueprints/Common/GameInstance_BAL.GameInstance_BAL_C|GetMatchData _asgame_instance_bal))))))
  (Class|SaveandLoadFiles|SaveJsontoFile _output_get)
  ;;[1 0.02348 0] Save the file data and try to send to server by http request
  (bind _returnvalue (UserInterface|CreateWidget "/Game/HUD/Menu/W_ShowScore.W_ShowScore_C"))
  (bind _output_get_2 (Variables|Game|SetShowScoreWidget _returnvalue))
  (UserInterface|Viewport|AddtoViewport _output_get_2 0))

(event Custom|On%20Preparation
  ;[1 1 1] On Preparation Event that calls all clients to set their variables
  (for _array_element (Variables|/Script/Engine.GameStateBase|GetPlayerArray (Game|GetGameState))
    (bind _aspstate (Utilities|Casting|CastToPState _array_element))
    (CallFunction|PreparationTimeBegin)
    (CallFunction|SetSpawnIntervalTimeA)
    (CallFunction|SetSpawnIntervalTimeB)
    (Default|PreparationMatch _aspstate (Variables|Spawn|GetSpawn%20Index%201) (Variables|Spawn|GetSpawn%20Index%202) (Variables|Spawn|GetSpawn%20Index%203) (Variables|Spawn|GetSpawn%20Index%204) "417.799988,-690.000000,-200.000000" (Variables|Game|GetSpawn%20Interval%20A) (Variables|Game|GetSpawn%20Interval%20B) (Variables|Spawn|GetSpawn%20Quantity%20A1) (Variables|Spawn|GetSpawn%20Quantity%20B1) (Variables|Game|GetPreparation%20Time))))

(event Custom|Add%20Score%20To%20Score%20Holder
  ;[1 1 1] Adds score to the score holder
  (Default|SetPlayerScore (Variables|Actors|GetP1ScoreActor))
  (Default|SetPlayerScore (Variables|Actors|GetP2Score%20Actor)))

(event Custom|Preparation%20Time%20Begin
  ;[1 1 1] Binding timer for preparation phase where players will have a time to choose a spot for their recipient
  (bind _returnvalue (Utilities|Time|SetTimerbyEvent (delegate Custom|Preparation%20Time%20End) (Variables|Game|GetPreparation%20Time))))

(event EventBeginPlay
  ;[1 1 1] All the set up for the match
  (CallFunction|GetPlayersScores)
  (CallFunction|SetScoresActors)
  (bind _returnvalue (Game|SpawnActorfromClass "/Game/Blueprints/Common/BlueprintHttpActor.BlueprintHttpActor_C" (Math|Conversions|ToTransform(Vector) (Math|Vector|MakeVector 0.0 0.0 0.0)) "Undefined" 0 0))
  (Variables|Actors|SetHttp%20Actor _returnvalue)
  (Variables|Game|SetRecipient%202 0)
  (Utilities|FlowControl|Delay 0.2)
  (bind _asgame_instance_bal (Utilities|Casting|CastToGameInstance_BAL (Game|GetGameInstance)))
  (Variables|Game|SetRounds (Variables|/Game/Blueprints/Common/GameInstance_BAL.GameInstance_BAL_C|GetRounds _asgame_instance_bal))
  (Variables|Spawn|SetSpawn%20Quantity%20A1 (.no_coop_points (Utilities|Struct|BreakMatchData (Variables|/Game/Blueprints/Common/GameInstance_BAL.GameInstance_BAL_C|GetMatchData _asgame_instance_bal))))
  (Variables|Spawn|SetSpawn%20Quantity%20B1 (.coop_points (Utilities|Struct|BreakMatchData (Variables|/Game/Blueprints/Common/GameInstance_BAL.GameInstance_BAL_C|GetMatchData _asgame_instance_bal))))
  (Variables|Game|SetBotStrategy (.strategy (Utilities|Struct|BreakMatchData (Variables|/Game/Blueprints/Common/GameInstance_BAL.GameInstance_BAL_C|GetMatchData _asgame_instance_bal))))
  (CallFunction|OnPre-preparationStart)
  (CallFunction|PreparationTimeBegin)
  (CallFunction|SpawnFallingObjects (Variables|Spawn|GetSpawn%20Quantity%20A1) (Variables|Spawn|GetSpawn%20Quantity%20B1)))

(fn ConstructionScript)

(fn SetRoundData
  (params (Game%20Instance :type Game%20Instance%20BAL%20Object%20Reference))
  (return (Utilities|Struct|MakeRoundData (+ (- (Variables|/Game/Blueprints/Common/GameInstance_BAL.GameInstance_BAL_C|GetMax%20Rounds Game%20Instance) (Variables|/Game/Blueprints/Common/GameInstance_BAL.GameInstance_BAL_C|GetRounds Game%20Instance)) 1) (Variables|Game|GetP1RoundScore) (Variables|Game|GetP2RoundScore) (Variables|Game|GetRecipient%201) (Variables|Game|GetRecipient%202))))

(fn SetScoresbyRound
  (params (P1RoundScore :type Integer) (P2RoundScore :type Integer))
  (Variables|Game|SetP1RoundScore P1RoundScore)
  (Variables|Game|SetP2RoundScore P2RoundScore))

(fn SetTotalScore
  (bind _asgame_instance_bal (Utilities|Casting|CastToGameInstance_BAL (Game|GetGameInstance)))
  (Variables|/Game/Blueprints/Common/GameInstance_BAL.GameInstance_BAL_C|SetP1TotalScore _asgame_instance_bal 0)
  (Variables|/Game/Blueprints/Common/GameInstance_BAL.GameInstance_BAL_C|SetP2TotalScore _asgame_instance_bal 0)
  (for _array_element (Variables|/Game/Blueprints/Common/GameInstance_BAL.GameInstance_BAL_C|GetRoundData _asgame_instance_bal)
    (Variables|/Game/Blueprints/Common/GameInstance_BAL.GameInstance_BAL_C|SetP1TotalScore _asgame_instance_bal (+ (Variables|/Game/Blueprints/Common/GameInstance_BAL.GameInstance_BAL_C|GetP1TotalScore _asgame_instance_bal) (.player1Score (Utilities|Struct|BreakRoundData _array_element))))
    (Variables|/Game/Blueprints/Common/GameInstance_BAL.GameInstance_BAL_C|SetP2TotalScore _asgame_instance_bal (+ (Variables|/Game/Blueprints/Common/GameInstance_BAL.GameInstance_BAL_C|GetP2TotalScore _asgame_instance_bal) (.player2Score (Utilities|Struct|BreakRoundData _array_element))))))

(fn GetPlayersScores
  (bind _asgame_instance_bal (Utilities|Casting|CastToGameInstance_BAL (Game|GetGameInstance)))
  (Variables|Game|SetPlayer1Score (Variables|/Game/Blueprints/Common/GameInstance_BAL.GameInstance_BAL_C|GetP1TotalScore _asgame_instance_bal))
  (Variables|Game|SetPlayer2Score (Variables|/Game/Blueprints/Common/GameInstance_BAL.GameInstance_BAL_C|GetP2TotalScore _asgame_instance_bal)))

(fn SetScoresActors
  (bind _outactors (Actor|GetAllActorsOfClass "/Game/Blueprints/Common/ScoreHolder.ScoreHolder_C"))
  (for _array_element _outactors
    (if (Utilities|Enum|Equal(Enum) (Utilities|GetDisplayName _array_element) "FirstScoreHolder")
      (Variables|Actors|SetP1ScoreActor _array_element)
      (else
        (Variables|Actors|SetP2Score%20Actor _array_element)))))